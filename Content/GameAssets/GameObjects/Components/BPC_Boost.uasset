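; Boost component for BP_Mech_Base that launches the mech along its movement input when IA_Boost fires, spending a clamped boost meter.
; Boosts require enough meter and nonzero velocity, with separate air and ground strengths; air boosts add upward lift.
; A DoOnce gates repeats while gravity or ground friction is briefly lowered.
; Each boost starts a looping refill timer, plays a sound and calls OnBoost.
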(event `self.ReceiveBeginPlay`
  (bind _asbp_mech_base (cast `/Game/GameAssets/GameObjects/Characters/BP_Mech_Base` (`self.GetOwner`)))
  (set `self.Owner` _asbp_mech_base)
  (set `self.CurrentBoost` (`self.MaxBoost`)))

(event `EnhancedInput|/Game/GameAssets/Inputs/IA_Boost`
  (params (ActionValue :type Boolean) (ElapsedSeconds :type "Float (double-precision)") (TriggeredSeconds :type "Float (double-precision)") (InputAction :type "InputAction Object Reference" :default "/Game/GameAssets/Inputs/IA_Boost.IA_Boost"))
  (bind _charactermovement (`Character.CharacterMovement` (`self.Owner`)))
  (bind _charactermovement_2 (`Character.CharacterMovement` (`self.Owner`)))
  (:`Triggered`
    (if (and (>= (`self.CurrentBoost`) (`self.BoostSubtraction`)) (!= (`MovementComponent.Velocity` (`Character.CharacterMovement` (`self.Owner`))) (0.0 0.0 0.0)))
      (`/Engine/EditorBlueprintResources/StandardMacros.DoOnce` false :!label _label
        (:`Completed`
          (bind _returnvalue (`KismetSystemLibrary.K2_SetTimerDelegate` (`|CreateDelegate` :!event `RefillTick`) 0.1 true false 2.0))
          (set `self.RefillTickTimer` _returnvalue)
          (`self.Boost`)
          (if (`NavMovementComponent.IsFalling` (`Character.CharacterMovement` (`self.Owner`)))
            (set `CharacterMovementComponent.GravityScale` 0.0 _charactermovement_2)
            (`KismetSystemLibrary.Delay` 0.25)
            (set `CharacterMovementComponent.GravityScale` 4.0 _charactermovement)
            (goto _label :!via `Reset`)
            (else
              (set `CharacterMovementComponent.GroundFriction` 0.4 _charactermovement_2)
              (`KismetSystemLibrary.Delay` 0.2)
              (set `CharacterMovementComponent.GroundFriction` 8.0 _charactermovement)
              (goto _label :!via `Reset`))))))))

(event `Boost`
  (if (`NavMovementComponent.IsFalling` (`Character.CharacterMovement` (`self.Owner`)))
    (bind _direction (`self.GetDirection`))
    (bind (_returnvalue_x _returnvalue_y) (`KismetMathLibrary.BreakVector` (* _direction (`self.AirBoostValue`))))
    (`Character.LaunchCharacter` (`self.Owner`) (`KismetMathLibrary.MakeVector` _returnvalue_x _returnvalue_y 100.0) true true)
    (else
      (bind _direction_2 (`self.GetDirection`))
      (bind (_returnvalue_x_2 _returnvalue_y_2) (`KismetMathLibrary.BreakVector` (* _direction_2 (`self.GroundBoostValue`))))
      (`Character.LaunchCharacter` (`self.Owner`) (`KismetMathLibrary.MakeVector` _returnvalue_x_2 _returnvalue_y_2) true false)))
  (`self.ChangeBoostValue` (* (`self.BoostSubtraction`) -1))
  (`self.OnBoost`)
  (`GameplayStatics.PlaySound2D` "/Game/GameAssets/Audio/boost.boost" 1.0 2.0 0.0 null null))

(event `ChangeBoostValue`
  (params (Value :type Integer))
  (set `self.CurrentBoost` (`KismetMathLibrary.Clamp` (+ Value (`self.CurrentBoost`)) 0 (`self.MaxBoost`))))

(event `RefillTick`
  (`self.ChangeBoostValue` 10)
  (if (== (`self.CurrentBoost`) (`self.MaxBoost`))
    (`KismetSystemLibrary.K2_ClearAndInvalidateTimerHandle` (`self.RefillTickTimer`))))

(fn `GetDirection`
  (returns (Direction :type "Vector Structure"))
  (bind _owner (`self.Owner`))
  (bind (_movementaxis_x _movementaxis_y) (`KismetMathLibrary.BreakVector2D` (`/Game/GameAssets/GameObjects/Characters/BP_Mech_Base.MovementAxis` _owner)))
  (return (`KismetMathLibrary.Normal` (+ (* (`Actor.GetActorRightVector` _owner) _movementaxis_x) (* _movementaxis_y (`Actor.GetActorForwardVector` _owner))))))