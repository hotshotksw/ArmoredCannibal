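; BPC_Health is an actor component that tracks health for its owning BP_Mech_Base and starts it at MaxHealth on BeginPlay.
; TakeDamage only applies when the owner's EntityTags contain the Entity.Damageable gameplay tag; it subtracts without clamping, then calls OnDamageTaken, plus OnDeath at zero or below.
; HealDamage adds health clamped between zero and MaxHealth, with no tag check or notification.
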(event `self.ReceiveBeginPlay`
  (bind _asbp_mech_base (cast `/Game/GameAssets/GameObjects/Characters/BP_Mech_Base` (`self.GetOwner`)))
  (set `self.Owner` _asbp_mech_base)
  (set `self.Health` (`self.MaxHealth`)))

(event `TakeDamage`
  (params (Damage :type "Float (double-precision)"))
  (if (`BlueprintGameplayTagLibrary.HasTag` (`/Game/GameAssets/GameObjects/Characters/BP_Mech_Base.EntityTags` (`self.Owner`)) (struct :`TagName` "GameTags.Entity.Damageable"))
    (bind _output_get (set `self.Health` (- (`self.Health`) Damage)))
    (`self.OnDamageTaken`)
    (if (<= _output_get 0.0)
      (`self.OnDeath`))))

(event `HealDamage`
  (params (Heal :type "Float (double-precision)"))
  (set `self.Health` (`KismetMathLibrary.FClamp` (+ Heal (`self.Health`)) 0.0 (`self.MaxHealth`))))