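; BP_InteractableAudio is a level object that plays a sound at its location when an allowed actor enters its collision box.
; While interactable, a box overlap compares the other actor's exact class against the InteractableEntities list.
; The first match disables interaction and plays Audio at reduced volume.
; After the loop, matched or not, a ReactivateDelay delay sets Interactable back to true, acting as a cooldown.
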(event `self.BoxCollision.OnComponentBeginOverlap`
  (params (OverlappedComponent :type "PrimitiveComponent Object Reference") (OtherActor :type "Actor Object Reference") (OtherComp :type "PrimitiveComponent Object Reference") (OtherBodyIndex :type Integer) (bFromSweep :type Boolean) (SweepResult :type "HitResult Structure (by ref)"))
  (if (`self.Interactable`)
    (for _array_element (`self.InteractableEntities`)
      (if (== _array_element (`GameplayStatics.GetObjectClass` OtherActor))
        (set `self.Interactable` false)
        (`GameplayStatics.PlaySoundAtLocation` (`self.Audio`) (`self.K2_GetActorLocation`) (struct) 0.5 1.0 0.0 null null null null)
        (break)))
    (`KismetSystemLibrary.Delay` (`self.ReactivateDelay`))
    (set `self.Interactable` true)))

(fn `UserConstructionScript`)