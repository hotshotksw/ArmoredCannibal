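; Encounter manager actor that links a group of enemies and signals when all of them are dead.
; On BeginPlay it binds to each enemy controller's target-spotted event and each health component's damage and death events.
; AlertEnemies puts every enemy's controller on alert.
; Deaths shrink the list, firing OnEncounterFinished when empty, otherwise playing a radio cue and a randomly picked death voiceline from the remaining enemies.
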(event `self.ReceiveBeginPlay`
  (bind _bpc_health (`/Game/GameAssets/GameObjects/Characters/BP_Mech_Base.BPC_Health` (`self.CurrentEnemy`)))
  (for _array_element (`self.Enemies`)
    (bind _output_get (set `self.CurrentEnemy` _array_element))
    (bind _asbp_enemy_controller (cast `/Game/GameAssets/GameObjects/Characters/BP_Enemy_Controller` (`AIBlueprintHelperLibrary.GetAIController` _output_get)))
    (add `/Game/GameAssets/GameObjects/Characters/BP_Enemy_Controller.OnTargetSpotted` _asbp_enemy_controller (`|CreateDelegate` :!event `AlertEnemies`))
    (add `/Game/GameAssets/GameObjects/Components/BPC_Health.OnDamageTaken` _bpc_health (`|CreateDelegate` :!event `AlertEnemies`))
    (add `/Game/GameAssets/GameObjects/Components/BPC_Health.OnDeath` _bpc_health (`|CreateDelegate` :!event `OnEnemyDeath`))))

(event `AlertEnemies`
  (for _array_element (`self.Enemies`)
    (bind _asbp_enemy_controller (cast `/Game/GameAssets/GameObjects/Characters/BP_Enemy_Controller` (`AIBlueprintHelperLibrary.GetAIController` _array_element)))
    (`/Game/GameAssets/GameObjects/Characters/BP_Enemy_Controller.Alert` _asbp_enemy_controller)))

(event `OnEnemyDeath`
  (params (DeadMech :type "/Game/GameAssets/GameObjects/Characters/BP_Mech_Base Object Reference"))
  (bind _enemies (`self.Enemies`))
  (bind _outitem (`KismetArrayLibrary.Array_Random` _enemies))
  (bind _outitem_2 (`KismetArrayLibrary.Array_Random` (`/Game/GameAssets/GameObjects/Characters/BP_Mech_Enemy.DeathVoicelines` _outitem)))
  (for _array_element (`self.Enemies`)
    (if (== DeadMech _array_element)
      (`KismetArrayLibrary.Array_RemoveItem` (`self.Enemies`) _array_element)
      (break)))
  (if (== (`KismetArrayLibrary.Array_Length` _enemies) 0)
    (`self.OnEncounterFinished`)
    (else
      (`/Engine/EditorBlueprintResources/StandardMacros.IsValid` _outitem
        (:`Is Valid`
          (if (not (`BlueprintGameplayTagLibrary.HasTag` (`/Game/GameAssets/GameObjects/Characters/BP_Mech_Base.EntityTags` _outitem) (struct :`TagName` "GameTags.Entity.Dead")))
            (`KismetSystemLibrary.Delay` 0.5)
            (`GameplayStatics.PlaySound2D` "/Game/GameAssets/Audio/radio_on.radio_on" 0.25 1.0 0.0 null null)
            (`KismetSystemLibrary.Delay` 0.5)
            (`/Engine/EditorBlueprintResources/StandardMacros.IsValid` _outitem_2
              (:`Is Valid`
                (`GameplayStatics.PlaySound2D` _outitem_2 0.25 1.0 0.0 null null)
                (`KismetSystemLibrary.PrintString` "AUDIO PLAYED")))))))))

(fn `UserConstructionScript`)