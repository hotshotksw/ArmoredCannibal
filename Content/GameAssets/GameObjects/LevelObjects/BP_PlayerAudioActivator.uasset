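; BP_PlayerAudioActivator is a level trigger volume that plays an assigned sound once when the player mech enters it.
; The box overlap casts to BP_Mech_Player, passes a DoOnce, waits PlayDelay, then spawns Audio attached to the player's capsule with environment attenuation, so the sound follows the player.
; A few leftover nodes, including a play-at-location call, are disconnected and never run.
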(event `self.BoxCollision.OnComponentBeginOverlap`
  (params (OverlappedComponent :type "PrimitiveComponent Object Reference") (OtherActor :type "Actor Object Reference") (OtherComp :type "PrimitiveComponent Object Reference") (OtherBodyIndex :type Integer) (bFromSweep :type Boolean) (SweepResult :type "HitResult Structure (by ref)"))
  (bind _asbp_mech_player (cast `/Game/GameAssets/GameObjects/Characters/BP_Mech_Player` OtherActor))
  (`/Engine/EditorBlueprintResources/StandardMacros.DoOnce` false
    (:`Completed`
      (`KismetSystemLibrary.Delay` (`self.PlayDelay`))
      (`GameplayStatics.SpawnSoundAttached` (`self.Audio`) (`Character.CapsuleComponent` _asbp_mech_player) "None" (`self.K2_GetActorLocation` _asbp_mech_player) (struct) "KeepWorldPosition" false 1.0 1.0 0.0 "/Game/GameAssets/Audio/SA_Environment.SA_Environment" null))))

(fn `UserConstructionScript`)