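; Level door that slides or swings its mesh between its starting transform and EndLocation via the DoorLerp timeline, with positional sounds.
; A mech's capsule entering the box opens it if the mech is tagged Interactable, guarded by a DoOnce; any mech capsule leaving resets the guard and reverses the timeline.
; RequiresActivation disables these triggers until OpenDoor clears it and opens the door immediately.
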(event `self.ReceiveBeginPlay`
  (set `self.StartLocation` (`SceneComponent.GetRelativeTransform` (`self.StaticMesh`))))

(event `OpenDoor`
  (set `self.RequiresActivation` false)
  (`GameplayStatics.PlaySoundAtLocation` (`self.ActivationSound`) (`SceneComponent.K2_GetComponentLocation` (`self.StaticMesh`)) (struct) 0.5 1.0 0.0 "/Game/GameAssets/Audio/SA_Environment.SA_Environment" null null null :!label _label)
  (bind (_direction _lerptime) (`Timeline|DoorLerp` :!label _label_2)
    (:`Update`
      (`SceneComponent.K2_SetRelativeTransform` (`self.StaticMesh`) (`KismetMathLibrary.TLerp` (`self.StartLocation`) (`self.EndLocation`) _lerptime) false false))
    (:`Finished`
      (`GameplayStatics.PlaySoundAtLocation` (`self.CloseSound`) (`SceneComponent.K2_GetComponentLocation` (`self.StaticMesh`)) (struct) 2.5 1.0 0.0 "/Game/GameAssets/Audio/SA_Environment.SA_Environment" null null null))))

(event `self.BoxCollision.OnComponentBeginOverlap`
  (params (OverlappedComponent :type "PrimitiveComponent Object Reference") (OtherActor :type "Actor Object Reference") (OtherComp :type "PrimitiveComponent Object Reference") (OtherBodyIndex :type Integer) (bFromSweep :type Boolean) (SweepResult :type "HitResult Structure (by ref)"))
  (if (not (`self.RequiresActivation`))
    (bind _asbp_mech_base (cast `/Game/GameAssets/GameObjects/Characters/BP_Mech_Base` OtherActor))
    (cast `CapsuleComponent` OtherComp)
    (if (`BlueprintGameplayTagLibrary.HasTag` (`/Game/GameAssets/GameObjects/Characters/BP_Mech_Base.EntityTags` _asbp_mech_base) (struct :`TagName` "GameTags.Entity.Interactable"))
      (`/Engine/EditorBlueprintResources/StandardMacros.DoOnce` false :!label _label_3
        (:`Completed`
          (goto _label))))))

(event `self.BoxCollision.OnComponentEndOverlap`
  (params (OverlappedComponent :type "PrimitiveComponent Object Reference") (OtherActor :type "Actor Object Reference") (OtherComp :type "PrimitiveComponent Object Reference") (OtherBodyIndex :type Integer))
  (if (not (`self.RequiresActivation`))
    (cast `/Game/GameAssets/GameObjects/Characters/BP_Mech_Base` OtherActor)
    (cast `CapsuleComponent` OtherComp)
    (`|ExecutionSequence`
      (:`then_0`
        (goto _label_3 :!via `Reset`))
      (:`then_1`
        (`GameplayStatics.PlaySoundAtLocation` (`self.ActivationSound`) (`SceneComponent.K2_GetComponentLocation` (`self.StaticMesh`)) (struct) 0.5 1.0 0.0 "/Game/GameAssets/Audio/SA_Environment.SA_Environment" null null null)
        (goto _label_2 :!via `Reverse`)))))

(fn `UserConstructionScript`)