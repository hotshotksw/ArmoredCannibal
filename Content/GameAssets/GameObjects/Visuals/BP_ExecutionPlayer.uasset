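; Execution sequence actor that plays a forward finisher between the player mech and an enemy mech, then destroys itself.
; It unpossesses the enemy's AI, plays the player montage and has the enemy play its own, placed ahead of the player.
; A Gameplay Cameras animation runs with this actor as view target.
; After the montage, it triggers the enemy's death, restores the view and movement tag, then removes player invincibility after a delay.
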(event `self.ReceiveBeginPlay`
  (bind _asbp_mech_player (cast `/Game/GameAssets/GameObjects/Characters/BP_Mech_Player` (`GameplayStatics.GetPlayerCharacter` 0)))
  (set `self.Executer` _asbp_mech_player))

(event `PlayCameraAnimation`
  (params (ExecutedEnemy :type "/Game/GameAssets/GameObjects/Characters/BP_Mech_Base Object Reference"))
  (bind _returnvalue (`GameplayStatics.GetPlayerController` 0))
  (bind _executer (`self.Executer`))
  (bind _output_get (set `self.Executee` ExecutedEnemy))
  (`Controller.UnPossess` (`AIBlueprintHelperLibrary.GetAIController` _output_get))
  (bind _returnvalue_2 (`Character.PlayAnimMontage` (`self.Executer`) "/Game/GameAssets/GameObjects/Characters/_ANIMATIONS/Executions/ExecutionForward_AC_Montage.ExecutionForward_AC_Montage" 1.0 "None"))
  (bind _asbp_mech_enemy (cast `/Game/GameAssets/GameObjects/Characters/BP_Mech_Enemy` (`self.Executee`)))
  (`/Game/GameAssets/GameObjects/Characters/BP_Mech_Enemy.Execute` _asbp_mech_enemy "/Game/GameAssets/GameObjects/Characters/_ANIMATIONS/Executions/ExecutionForward_01_Montage.ExecutionForward_01_Montage" (`KismetMathLibrary.MakeTransform` (+ (`self.K2_GetActorLocation` _executer) (* (`self.GetActorForwardVector` _executer) 200.0)) (`KismetMathLibrary.FindLookAtRotation` (`self.K2_GetActorLocation` (`self.Executee`)) (`self.K2_GetActorLocation` _executer)) (`self.GetActorScale3D` (`self.Executee`))))
  (bind _returnvalue_3 (`GameplayCamerasSubsystem.PlayCameraAnimation` :`self` (subsystem `GameplayCamerasSubsystem`) :`PlayerController` _returnvalue :`Sequence` "/Game/GameAssets/Levels/Sequences/CAS_Execute_Fwd.CAS_Execute_Fwd"))
  (`PlayerController.SetViewTargetWithBlend` _returnvalue self 0.0 "VTBlend_Linear" 0.0 false)
  (`KismetSystemLibrary.Delay` _returnvalue_2)
  (`self.EndCameraAnimation`))

(event `EndCameraAnimation`
  (bind _returnvalue (`GameplayStatics.GetPlayerController` 0))
  (bind _entitytags (`/Game/GameAssets/GameObjects/Characters/BP_Mech_Base.EntityTags` (`self.Executer`)))
  (bind _asbp_mech_enemy (cast `/Game/GameAssets/GameObjects/Characters/BP_Mech_Enemy` (`self.Executee`)))
  (`/Game/GameAssets/GameObjects/Characters/BP_Mech_Enemy.ExecutedDeath` _asbp_mech_enemy)
  (`GameplayCamerasSubsystem.StopCameraAnimation` (subsystem `GameplayCamerasSubsystem`) _returnvalue (stale `PlayCameraAnimation` _returnvalue_3) false)
  (`PlayerController.SetViewTargetWithBlend` _returnvalue (`GameplayStatics.GetPlayerCharacter` 0) 0.0 "VTBlend_Linear" 0.0 false)
  (`BlueprintGameplayTagLibrary.AddGameplayTag` _entitytags (struct :`TagName` "GameTags.Entity.Moveable"))
  (`KismetSystemLibrary.Delay` 1.0)
  (`BlueprintGameplayTagLibrary.RemoveGameplayTag` _entitytags (struct :`TagName` "GameTags.Entity.Invincible"))
  (`self.K2_DestroyActor`))

(fn `UserConstructionScript`)