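; BP_CamAnimPlayer is a temporary actor that drives the camera during an enemy execution.
; PlayCameraAnimation removes movement tags from enemy and player plus the player's damageable tag, plays the forward-execution sequence through GameplayCamerasSubsystem, and becomes the view target.
; EndCameraAnimation stops the sequence, returns view to the player, restores only the player's tags, then destroys the actor after a short delay.
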(event `PlayCameraAnimation`
  (params (ExecutedEnemy :type "/Game/GameAssets/GameObjects/Characters/BP_Mech_Enemy Object Reference"))
  (bind _returnvalue (`GameplayStatics.GetPlayerController` 0))
  (`BlueprintGameplayTagLibrary.RemoveGameplayTag` (`/Game/GameAssets/GameObjects/Characters/BP_Mech_Base.EntityTags` ExecutedEnemy) (struct :`TagName` "GameTags.Entity.Moveable"))
  (bind _asbp_mech_player (cast `/Game/GameAssets/GameObjects/Characters/BP_Mech_Player` (`GameplayStatics.GetPlayerCharacter` 0)))
  (bind _entitytags (`/Game/GameAssets/GameObjects/Characters/BP_Mech_Base.EntityTags` _asbp_mech_player))
  (`BlueprintGameplayTagLibrary.RemoveGameplayTag` _entitytags (struct :`TagName` "GameTags.Entity.Moveable"))
  (`BlueprintGameplayTagLibrary.RemoveGameplayTag` _entitytags (struct :`TagName` "GameTags.Entity.Damageable"))
  (bind _returnvalue_2 (`GameplayCamerasSubsystem.PlayCameraAnimation` :`self` (subsystem `GameplayCamerasSubsystem`) :`PlayerController` _returnvalue :`Sequence` "/Game/GameAssets/Levels/Sequences/CAS_Execute_Fwd.CAS_Execute_Fwd"))
  (`PlayerController.SetViewTargetWithBlend` _returnvalue self 0.0 "VTBlend_Linear" 0.0 false))

(event `EndCameraAnimation`
  (bind _returnvalue (`GameplayStatics.GetPlayerController` 0))
  (`GameplayCamerasSubsystem.StopCameraAnimation` (subsystem `GameplayCamerasSubsystem`) _returnvalue (stale `PlayCameraAnimation` _returnvalue_2) false)
  (`PlayerController.SetViewTargetWithBlend` _returnvalue (`GameplayStatics.GetPlayerCharacter` 0) 0.0 "VTBlend_Linear" 0.0 false)
  (bind _asbp_mech_player (cast `/Game/GameAssets/GameObjects/Characters/BP_Mech_Player` (`GameplayStatics.GetPlayerCharacter` 0)))
  (bind _entitytags (`/Game/GameAssets/GameObjects/Characters/BP_Mech_Base.EntityTags` _asbp_mech_player))
  (`BlueprintGameplayTagLibrary.AddGameplayTag` _entitytags (struct :`TagName` "GameTags.Entity.Moveable"))
  (`BlueprintGameplayTagLibrary.AddGameplayTag` _entitytags (struct :`TagName` "GameTags.Entity.Damageable"))
  (`KismetSystemLibrary.Delay` 1.0)
  (`self.K2_DestroyActor`))

(fn `UserConstructionScript`)