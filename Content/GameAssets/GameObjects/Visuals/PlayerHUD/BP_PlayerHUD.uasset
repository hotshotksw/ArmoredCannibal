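; Player HUD actor that owns the main HUD widget and a hit-effect overlay, adding both to the viewport on BeginPlay.
; FadeHUD toggles visibility by playing the HUD's Fade animation forward or in reverse from its current time, so interrupted fades continue from that point.
; PlayHit plays the overlay's Hit animation, restarting slightly past its start if it is already underway.
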(event `self.ReceiveBeginPlay`
  (bind _returnvalue (`|CreateWidget` "/Game/GameAssets/GameObjects/Visuals/PlayerHUD/W_HUD.W_HUD_C" (`GameplayStatics.GetPlayerController` 0)))
  (bind _output_get (set `self.UI` _returnvalue))
  (`UserWidget.AddToViewport` _output_get 0)
  (bind _returnvalue_2 (`|CreateWidget` "/Game/GameAssets/GameObjects/Visuals/W_HitEffect.W_HitEffect_C"))
  (bind _output_get_2 (set `self.DamageUI` _returnvalue_2))
  (`UserWidget.AddToViewport` _output_get_2 0))

(event `self.ReceiveTick`
  (params (DeltaSeconds :type "Float (single-precision)")))

(fn `FadeHUD`
  (if (`self.VisibleHUD`)
    (bind _ui (`self.UI`)
      (:`then`
        (bind _fade (`/Game/GameAssets/GameObjects/Visuals/PlayerHUD/W_HUD.Fade` _ui))
        (bind _returnvalue (`UserWidget.GetAnimationCurrentTime` _ui _fade))
        (`UserWidget.PlayAnimation` _ui _fade _returnvalue 1 "Reverse" 1.0 false)
        (set `self.VisibleHUD` false))
      (:`else`))
    (else
      (bind _ui_2 (`self.UI`)
        (:`then`
          (`UserWidget.PlayAnimation` _ui_2 (`/Game/GameAssets/GameObjects/Visuals/PlayerHUD/W_HUD.Fade` _ui_2) _returnvalue 1 "Forward" 1.25 false)
          (set `self.VisibleHUD` true))
        (:`else`)))))

(fn `PlayHit`
  (bind _damageui (`self.DamageUI`))
  (bind _damageui_2 (`self.DamageUI`))
  (bind _damageui_3 (`self.DamageUI`))
  (if (<= (`UserWidget.GetAnimationCurrentTime` _damageui_2 (`/Game/GameAssets/GameObjects/Visuals/W_HitEffect.Hit` _damageui_2)) 0.0)
    (`UserWidget.PlayAnimation` _damageui_3 (`/Game/GameAssets/GameObjects/Visuals/W_HitEffect.Hit` _damageui_3) 0.0 1 "Forward" 1.0 false)
    (else
      (`UserWidget.PlayAnimation` _damageui (`/Game/GameAssets/GameObjects/Visuals/W_HitEffect.Hit` _damageui) 0.15 1 "Forward" 1.0 false))))

(fn `UserConstructionScript`)