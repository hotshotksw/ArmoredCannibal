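; BP_WeaponPickup is a pickup actor that displays a weapon and hands it to a mech that overlaps it.
; On BeginPlay it spawns the configured WeaponClass at its Sphere, enlarges it and attaches it there.
; When a BP_Mech_Base enters the Sphere, it restores normal weapon scale and sets the owner.
; It then adds that same instance to the primary or secondary weapon platform by weapon position and destroys itself.
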(event `self.ReceiveBeginPlay`
  (bind _returnvalue (`|SpawnActorFromClass` (`self.WeaponClass`) (`SceneComponent.K2_GetComponentToWorld` (`self.Sphere`)) "Undefined" "OverrideRootScale" null null))
  (bind _output_get (set `self.Weapon` _returnvalue))
  (`self.SetActorScale3D` _output_get (4.0 4.0 4.0))
  (`self.K2_AttachToComponent` (`self.Weapon`) (`self.Sphere`) "None" "KeepWorld" "KeepRelative" "KeepRelative" true))

(event `self.Sphere.OnComponentBeginOverlap`
  (params (OverlappedComponent :type "PrimitiveComponent Object Reference") (OtherActor :type "Actor Object Reference") (OtherComp :type "PrimitiveComponent Object Reference") (OtherBodyIndex :type Integer) (bFromSweep :type Boolean) (SweepResult :type "HitResult Structure (by ref)"))
  (bind _weapon (`self.Weapon`))
  (bind _asbp_mech_base (cast `/Game/GameAssets/GameObjects/Characters/BP_Mech_Base` OtherActor))
  (`self.SetActorScale3D` (`self.Weapon`) (1.0 1.0 1.0))
  (set `/Game/GameAssets/GameObjects/Weapons/BP_Weapon_B.WeaponOwner` _asbp_mech_base (`self.Weapon`))
  (bind _position (`/Game/GameAssets/GameObjects/Weapons/BP_Weapon_B.GetWeaponPosition` (`self.Weapon`)))
  (if (`|EnumEquality` _position "NewEnumerator0")
    (`/Game/GameAssets/GameObjects/Components/BPC_WeaponPlatform.Add Weapon` (`/Game/GameAssets/GameObjects/Characters/BP_Mech_Base.WeaponPlatform_Primary` _asbp_mech_base) _weapon)
    (else
      (`/Game/GameAssets/GameObjects/Components/BPC_WeaponPlatform.Add Weapon` (`/Game/GameAssets/GameObjects/Characters/BP_Mech_Base.WeaponPlatform_Secondary` _asbp_mech_base) _weapon)))
  (`self.K2_DestroyActor`))

(fn `UserConstructionScript`)