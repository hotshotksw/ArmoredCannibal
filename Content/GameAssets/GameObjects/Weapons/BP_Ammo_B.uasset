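; BP_Ammo_B is a projectile weapon round that damages mechs it hits.
; The construction script applies AmmoData to the projectile movement speed, lifespan and collision sphere radius.
; On sphere overlap with anything but its owner, it calls TakeDamage on a BP_Mech_Base's BPC_Health component, then destroys itself.
; Other non-owner overlaps also destroy it, and a mech lacking that component prints an error.
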(event `self.SphereCollision.OnComponentBeginOverlap`
  (params (OverlappedComponent :type "PrimitiveComponent Object Reference") (OtherActor :type "Actor Object Reference") (OtherComp :type "PrimitiveComponent Object Reference") (OtherBodyIndex :type Integer) (bFromSweep :type Boolean) (SweepResult :type "HitResult Structure (by ref)"))
  (bind (_ammodata_lifespan _ammodata_speed _ammodata_hitradius _ammodata_damage) (break `/Game/GameAssets/GameObjects/Weapons/ST_Ammo` (`self.AmmoData`)))
  (if (!= (`self.GetOwner`) OtherActor)
    (bind _asbp_mech_base (cast `/Game/GameAssets/GameObjects/Characters/BP_Mech_Base` OtherActor)
      (:`then`
        (bind _returnvalue (`self.GetComponentByClass` _asbp_mech_base "/Game/GameAssets/GameObjects/Components/BPC_Health.BPC_Health_C"))
        (`/Engine/EditorBlueprintResources/StandardMacros.IsValid` _returnvalue
          (:`Is Valid`
            (`/Game/GameAssets/GameObjects/Components/BPC_Health.TakeDamage` _returnvalue _ammodata_damage)
            (`self.K2_DestroyActor`))
          (:`Is Not Valid`
            (`KismetSystemLibrary.PrintString` "ERROR: FAILED TO FIND COMPONENT / TAKE DAMAGE")
            (`self.K2_DestroyActor`))))
      (:`CastFailed`
        (`self.K2_DestroyActor`)))))

(fn `UserConstructionScript`
  (bind _projectilemovement (`self.ProjectileMovement`))
  (bind (_ammodata_lifespan _ammodata_speed _ammodata_hitradius) (break `/Game/GameAssets/GameObjects/Weapons/ST_Ammo` (`self.AmmoData`)))
  (bind (_ammodata_lifespan_2 _ammodata_speed_2) (break `/Game/GameAssets/GameObjects/Weapons/ST_Ammo` (`self.AmmoData`)))
  (bind _output_get (set `ProjectileMovementComponent.InitialSpeed` _ammodata_speed_2 _projectilemovement))
  (set `ProjectileMovementComponent.MaxSpeed` _output_get _projectilemovement)
  (`self.SetLifeSpan` _ammodata_lifespan)
  (`SphereComponent.SetSphereRadius` (`self.SphereCollision`) _ammodata_hitradius true))