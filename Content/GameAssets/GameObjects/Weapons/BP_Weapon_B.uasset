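; BP_Weapon_B is a weapon Blueprint, apparently a base, that fires hitscan or projectile shots based on gameplay tags.
; UseWeapon plays fire audio, then either sphere-traces from the owner's camera to damage BPC_Health or spawns the ammo class at the barrel.
; Only a damaging trace or successful spawn spends ammo and returns the fire rate.
; UseAmmo skips InfiniteAmmo weapons and signals weapon destruction when ammo runs low.
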(fn `FireHitscan`
  (returns (ValidExecution :type Boolean))
  (bind (_hitscandata_range _hitscandata_damage) (break `/Game/GameAssets/GameObjects/Weapons/ST_Hitscan` (`self.HitscanData`)))
  (bind _hitscandata_range_2 (break `/Game/GameAssets/GameObjects/Weapons/ST_Hitscan` (`self.HitscanData`)))
  (bind _camera (`/Game/GameAssets/GameObjects/Characters/BP_Mech_Base.Camera` (`self.WeaponOwner`)))
  (bind _returnvalue (`SceneComponent.K2_GetComponentLocation` _camera))
  (bind _outhit (`KismetSystemLibrary.SphereTraceSingleForObjects` _returnvalue (+ _returnvalue (* (`KismetMathLibrary.GetForwardVector` (`SceneComponent.K2_GetComponentRotation` _camera)) _hitscandata_range_2)) 0.0 (`|MakeArray` "ObjectTypeQuery1" "ObjectTypeQuery3" :!type "EObjectTypeQuery Enum") false (`|MakeArray` (`self.WeaponOwner`) :!type "Actor Object Reference") "None" true (struct :`R` 1.0 :`A` 1.0) (struct :`G` 1.0 :`A` 1.0) 1.0))
  (`/Engine/EditorBlueprintResources/StandardMacros.IsValid` (`.HitActor` (`GameplayStatics.BreakHitResult` _outhit))
    (:`Is Valid`
      (bind _returnvalue_2 (`self.GetComponentByClass` (`.HitActor` (`GameplayStatics.BreakHitResult` _outhit)) "/Game/GameAssets/GameObjects/Components/BPC_Health.BPC_Health_C"))
      (`/Engine/EditorBlueprintResources/StandardMacros.IsValid` _returnvalue_2
        (:`Is Valid`
          (`/Game/GameAssets/GameObjects/Components/BPC_Health.TakeDamage` _returnvalue_2 _hitscandata_damage)
          (return true))
        (:`Is Not Valid`
          (return false))))
    (:`Is Not Valid`
      (return false))))

(fn `FireProjectile`
  (returns (ValidExecution :type Boolean))
  (bind (_weapondata_usecost _weapondata_firerate _weapondata_ammo) (break `/Game/GameAssets/GameObjects/Weapons/ST_Weapon` (`self.WeaponData`)))
  (bind _returnvalue (`|SpawnActorFromClass` _weapondata_ammo (`SceneComponent.K2_GetComponentToWorld` (`self.Barrel`)) "Undefined" "OverrideRootScale" (`self.WeaponOwner`) null))
  (`/Engine/EditorBlueprintResources/StandardMacros.IsValid` _returnvalue
    (:`Is Valid`
      (return true))))

(fn `UseAmmo`
  (params (UseCost :type Integer))
  (bind _returnvalue (- (`self.AmmoReserve`) UseCost))
  (if (not (`BlueprintGameplayTagLibrary.HasTag` (`self.WeaponTags`) (struct :`TagName` "GameTags.Weapon.InfiniteAmmo")))
    (set `self.AmmoReserve` _returnvalue)
    (if (<= _returnvalue 0)
      (`self.OnWeaponDestroyed`))))

(fn `UserConstructionScript`)

(fn `UseWeapon`
  (returns (Firerate :type "Float (double-precision)"))
  (bind (_weapondata_usecost _weapondata_firerate _weapondata_ammo _weapondata_fireaudio) (break `/Game/GameAssets/GameObjects/Weapons/ST_Weapon` (`self.WeaponData`)))
  (bind (_weapondata_usecost_2 _weapondata_firerate_2) (break `/Game/GameAssets/GameObjects/Weapons/ST_Weapon` (`self.WeaponData`)))
  (if (`KismetSystemLibrary.IsValidClass` _weapondata_ammo)
    (`GameplayStatics.PlaySoundAtLocation` _weapondata_fireaudio (`SceneComponent.K2_GetComponentLocation` (`self.Barrel`)) (struct) 1.0 1.0 0.0 "/Game/GameAssets/Audio/SA_Gun.SA_Gun" null null null)
    (if (`BlueprintGameplayTagLibrary.HasTag` (`self.WeaponTags`) (struct :`TagName` "GameTags.Weapon.Hitscan"))
      (bind _validexecution (`self.FireHitscan`))
      (if _validexecution
        (`self.UseAmmo` _weapondata_usecost_2 :!label _label)
        (return _weapondata_firerate_2))
      (else
        (bind _validexecution_2 (`self.FireProjectile`))
        (if _validexecution_2
          (goto _label))))))