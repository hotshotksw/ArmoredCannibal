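; BP_Claws is a melee claw weapon with a three-swing combo that lunges its owner along the camera direction.
; UseWeapon launches the owner with damped vertical pull and less force on each successive swing, plays that swing's montage and sets timers scaled to its length.
; SwingHit adds camera shake and fires a hitscan.
; The combo wraps after the third swing or resets when the montage-length timer expires uninterrupted.
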(fn `ResetSwingAnim`
  (set `self.CurrentSwing` 0))

(fn `SwingHit`
  (`LegacyCameraShake.StartLegacyCameraShake` (`GameplayStatics.GetPlayerCameraManager` 0) "/Game/GameAssets/GameObjects/Characters/BP_CameraShake.BP_CameraShake_C")
  (`self.FireHitscan`))

(fn `UserConstructionScript`
  (`parent.UserConstructionScript`))

(fn `UseWeapon`
  (returns (Firerate :type "Float (double-precision)"))
  (bind (_returnvalue_x _returnvalue_y _returnvalue_z) (`KismetMathLibrary.BreakVector` (`KismetMathLibrary.GetForwardVector` (`SceneComponent.K2_GetComponentRotation` (`/Game/GameAssets/GameObjects/Characters/BP_Mech_Base.ActiveCamera` (`self.WeaponOwner`))))))
  (`KismetSystemLibrary.K2_ClearAndInvalidateTimerHandle` (`self.SwingCountTimer`))
  (`BlueprintGameplayTagLibrary.AddGameplayTag` (`self.WeaponTags`) (struct :`TagName` "GameTags.Weapon.Firing"))
  (`Character.LaunchCharacter` (`self.WeaponOwner`) (* (`KismetMathLibrary.MakeVector` _returnvalue_x _returnvalue_y (* _returnvalue_z 0.4)) (/ 4000 (+ (`self.CurrentSwing`) 1))) true true)
  (bind _returnvalue (`Character.PlayAnimMontage` (`self.WeaponOwner`) (`|GetArrayItem` (`self.SwingAnims`) (`self.CurrentSwing`)) 1.0 "None"))
  (`KismetSystemLibrary.K2_SetTimerDelegate` (`|CreateDelegate` :!event `SwingHit`) (* _returnvalue 0.25))
  (bind _result (`/Engine/EditorBlueprintResources/StandardMacros.IncrementInt` (`self.CurrentSwing`))
    (:`  `
      (if (> _result 2)
        (set `self.CurrentSwing` 0)
        (else
          (set `self.CurrentSwing` _result)))
      (bind _returnvalue_2 (`KismetSystemLibrary.K2_SetTimer` null "ResetSwingAnim" _returnvalue))
      (set `self.SwingCountTimer` _returnvalue_2)
      (return (* _returnvalue 0.55)))))