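; BP_Mech_Enemy is an AI mech that runs a behavior tree, targets the player mech and carries two infinite-ammo machine guns.
; Successful primary fire, gated by the Moveable tag, sets a FiringWeapon tag and switches walk speed until a timer resets both.
; Low health tags it Staggered, and Execute removes Moveable and plays the supplied montage.
; Death turns it toward the player, plays a montage, then explodes, strips weapons and destroys it.
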(event `self.ReceiveBeginPlay`
  (`AIController.RunBehaviorTree` (`AIBlueprintHelperLibrary.GetAIController` self) "/Game/GameAssets/GameObjects/Characters/BT_MechEnemy.BT_MechEnemy")
  (`parent.ReceiveBeginPlay`)
  (bind _asbp_mech_player (cast `/Game/GameAssets/GameObjects/Characters/BP_Mech_Player` (`GameplayStatics.GetPlayerCharacter` 0)))
  (set `self.Target` _asbp_mech_player)
  (for _ (range 2)
    (bind _returnvalue (`|SpawnActorFromClass` "/Game/GameAssets/GameObjects/Weapons/BP_MG.BP_MG_C" (`self.GetTransform`) "Undefined" "MultiplyWithRoot" self null))
    (`BlueprintGameplayTagLibrary.AddGameplayTag` (`/Game/GameAssets/GameObjects/Weapons/BP_Weapon_B.WeaponTags` _returnvalue) (struct :`TagName` "GameTags.Weapon.InfiniteAmmo"))
    (`/Game/GameAssets/GameObjects/Components/BPC_WeaponPlatform.Add Weapon` (`self.WeaponPlatform_Primary`) _returnvalue)))

(event `self.BPC_Health.OnDeath`
  (params (DeadMech :type "/Game/GameAssets/GameObjects/Characters/BP_Mech_Base Object Reference"))
  (bind _weaponplatform_secondary (`self.WeaponPlatform_Secondary`))
  (bind _weaponplatform_primary (`self.WeaponPlatform_Primary`))
  (`/Engine/EditorBlueprintResources/StandardMacros.DoOnce` false
    (:`Completed`
      (`self.K2_SetActorRotation` (`KismetMathLibrary.FindLookAtRotation` (`self.K2_GetActorLocation`) (`self.K2_GetActorLocation` (`GameplayStatics.GetPlayerCharacter` 0))))
      (`BlueprintGameplayTagLibrary.AddGameplayTag` (`self.EntityTags`) (struct :`TagName` "GameTags.Entity.Dead"))
      (`self.DetachFromControllerPendingDestroy`)
      (`|PlayMontage` (`self.Mesh`) "/Game/GameAssets/GameObjects/Characters/_ANIMATIONS/Standard/Death_01_Montage.Death_01_Montage"
        (:`then`
          (bind _as_game_instance (cast `/Game/GameAssets/_GAME_INSTANCE` (`GameplayStatics.GetGameInstance`)))
          (`/Game/GameAssets/_GAME_INSTANCE.Impact` _as_game_instance)
          (`KismetSystemLibrary.Delay` 0.2)
          (`GameplayStatics.PlaySoundAtLocation` "/Game/GameAssets/Audio/impact_01.impact_01" (`self.K2_GetActorLocation`) (struct) 0.5 1.0 0.0 "/Game/GameAssets/Audio/SA_Environment.SA_Environment" null null null)
          (`NiagaraFunctionLibrary.SpawnSystemAtLocation` "/Game/GameAssets/GameObjects/Particles/NS_Explosion.NS_Explosion" (`SceneComponent.K2_GetComponentLocation` (`self.Mesh`)) (struct) (1.5 1.5 1.5))
          (`NiagaraFunctionLibrary.SpawnSystemAtLocation` "/Game/GameAssets/GameObjects/Particles/NS_Blood_Explosion.NS_Blood_Explosion" (`SceneComponent.K2_GetComponentLocation` (`self.Mesh`)))
          (`/Game/GameAssets/GameObjects/Components/BPC_WeaponPlatform.RemoveLeftWeapon` _weaponplatform_primary)
          (`/Game/GameAssets/GameObjects/Components/BPC_WeaponPlatform.RemoveRightWeapon` _weaponplatform_primary)
          (`/Game/GameAssets/GameObjects/Components/BPC_WeaponPlatform.RemoveLeftWeapon` _weaponplatform_secondary)
          (`/Game/GameAssets/GameObjects/Components/BPC_WeaponPlatform.RemoveRightWeapon` _weaponplatform_secondary)
          (`self.K2_DestroyActor`))))))

(event `FirePrimaryLeft`
  (bind _weaponplatform_primary (`self.WeaponPlatform_Primary`))
  (if (`BlueprintGameplayTagLibrary.HasTag` (`self.EntityTags`) (struct :`TagName` "GameTags.Entity.Moveable"))
    (bind _weapon_l (`/Game/GameAssets/GameObjects/Components/BPC_WeaponPlatform.Weapon_L` _weaponplatform_primary)
      (:`then`
        (bind _executed (`/Game/GameAssets/GameObjects/Components/BPC_WeaponPlatform.Fire` _weaponplatform_primary _weapon_l))
        (if _executed
          (`BlueprintGameplayTagLibrary.AddGameplayTag` (`self.EntityTags`) (struct :`TagName` "GameTags.Entity.FiringWeapon") :!label _label)
          (set `CharacterMovementComponent.MaxWalkSpeed` (`|GetArrayItem` (`self.MechSpeeds`) 1) (`self.CharacterMovement`))
          (`KismetSystemLibrary.K2_SetTimerDelegate` (delegate `ResetFiring`) 2.0)))
      (:`else`))))

(event `FirePrimaryRight`
  (bind _weaponplatform_primary (`self.WeaponPlatform_Primary`))
  (if (`BlueprintGameplayTagLibrary.HasTag` (`self.EntityTags`) (struct :`TagName` "GameTags.Entity.Moveable"))
    (bind _weapon_r (`/Game/GameAssets/GameObjects/Components/BPC_WeaponPlatform.Weapon_R` _weaponplatform_primary)
      (:`then`
        (bind _executed (`/Game/GameAssets/GameObjects/Components/BPC_WeaponPlatform.Fire` _weaponplatform_primary _weapon_r))
        (if _executed
          (goto _label)))
      (:`else`))))

(event `ResetFiring`
  (`BlueprintGameplayTagLibrary.RemoveGameplayTag` (`self.EntityTags`) (struct :`TagName` "GameTags.Entity.FiringWeapon"))
  (set `CharacterMovementComponent.MaxWalkSpeed` (`|GetArrayItem` (`self.MechSpeeds`) 2) (`self.CharacterMovement`)))

(event `self.BPC_Health.OnDamageTaken`
  (bind _bpc_health (`self.BPC_Health`))
  (if (<= (/ (`/Game/GameAssets/GameObjects/Components/BPC_Health.Health` _bpc_health) (`/Game/GameAssets/GameObjects/Components/BPC_Health.MaxHealth` _bpc_health)) 0.34)
    (`BlueprintGameplayTagLibrary.AddGameplayTag` (`self.EntityTags`) (struct :`TagName` "GameTags.Entity.Staggered"))))

(event `Execute`
  (params (ExecutionAnim :type "AnimMontage Object Reference") (ExecutionTransform :type "Transform Structure"))
  (`BlueprintGameplayTagLibrary.RemoveGameplayTag` (`self.EntityTags`) (struct :`TagName` "GameTags.Entity.Moveable"))
  (`|PlayMontage` (`self.Mesh`) ExecutionAnim))

(fn `UserConstructionScript`
  (`parent.UserConstructionScript`))