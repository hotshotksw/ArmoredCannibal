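; BP_Mech_Base is a mech character Blueprint with Enhanced Input movement, look, jump and crouch.
; Crouch zeroes ground friction for a slide, raises gravity, tags the entity and shrinks the capsule via a timeline, all reversed on release.
; CheckCanMove toggles input from the Moveable gameplay tag.
; Jump uses plain Jump/StopJumping in two duplicate handlers; landing resets a jump counter, but the boosted double-jump logic is disconnected.
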(event `EnhancedInput|/Game/Game/Inputs/IA_Movement`
  (params (ActionValue :type "Vector2D Structure") (ElapsedSeconds :type "Float (double-precision)") (TriggeredSeconds :type "Float (double-precision)") (InputAction :type "InputAction Object Reference" :default "/Game/Game/Inputs/IA_Movement.IA_Movement"))
  (:`Triggered`
    (`self.AddMovementInput` (`self.GetActorRightVector`) ActionValue_X)
    (`self.AddMovementInput` (`self.GetActorForwardVector`) ActionValue_Y)))

(event `EnhancedInput|/Game/Game/Inputs/IA_Crouch`
  (params (ActionValue :type Boolean) (ElapsedSeconds :type "Float (double-precision)") (TriggeredSeconds :type "Float (double-precision)") (InputAction :type "InputAction Object Reference" :default "/Game/Game/Inputs/IA_Crouch.IA_Crouch"))
  (bind _charactermovement (`self.CharacterMovement`))
  (bind _entitytags (`self.EntityTags`))
  (:`Triggered`
    (`BlueprintGameplayTagLibrary.AddGameplayTag` _entitytags (struct :`TagName` "GameTags.Entity.Crouching"))
    (if (!= (`CharacterMovementComponent.GroundFriction` (`self.CharacterMovement`)) 0.4)
      (set `CharacterMovementComponent.GroundFriction` 0.0 _charactermovement)
      (set `CharacterMovementComponent.GravityScale` 4.0 _charactermovement)
      (bind (_direction _crouchtime) (`Timeline|CrouchLerp` :!label _label)
        (:`Update`
          (`CapsuleComponent.SetCapsuleHalfHeight` (`self.CapsuleComponent`) (`KismetMathLibrary.Lerp` 110.0 25.0 _crouchtime) true)))))
  (:`Canceled`
    (`BlueprintGameplayTagLibrary.RemoveGameplayTag` _entitytags (struct :`TagName` "GameTags.Entity.Crouching") :!label _label_2)
    (set `CharacterMovementComponent.GroundFriction` 8.0 (`self.CharacterMovement`))
    (set `CharacterMovementComponent.GravityScale` 2.0 (`self.CharacterMovement`))
    (goto _label :!via `Reverse`))
  (:`Completed`
    (goto _label_2)))

(event `EnhancedInput|/Game/Game/Inputs/IA_Look`
  (params (ActionValue :type "Vector2D Structure") (ElapsedSeconds :type "Float (double-precision)") (TriggeredSeconds :type "Float (double-precision)") (InputAction :type "InputAction Object Reference" :default "/Game/Game/Inputs/IA_Look.IA_Look"))
  (:`Triggered`
    (`self.AddControllerYawInput` ActionValue_X)
    (`self.AddControllerPitchInput` ActionValue_Y)))

(event `EnhancedInput|/Game/Game/Inputs/IA_Jump`
  (params (ActionValue :type Boolean) (ElapsedSeconds :type "Float (double-precision)") (TriggeredSeconds :type "Float (double-precision)") (InputAction :type "InputAction Object Reference" :default "/Game/Game/Inputs/IA_Jump.IA_Jump"))
  (:`Triggered`
    (`self.Jump`))
  (:`Canceled`
    (`self.StopJumping` :!label _label_3))
  (:`Completed`
    (goto _label_3)))

(event `EnhancedInput|/Game/Game/Inputs/IA_Jump`
  (params (ActionValue :type Boolean) (ElapsedSeconds :type "Float (double-precision)") (TriggeredSeconds :type "Float (double-precision)") (InputAction :type "InputAction Object Reference" :default "/Game/Game/Inputs/IA_Jump.IA_Jump"))
  (:`Triggered`
    (`self.Jump`))
  (:`Canceled`
    (`self.StopJumping` :!label _label_4))
  (:`Completed`
    (goto _label_4)))

(event `self.OnLanded`
  (params (Hit :type "HitResult Structure (by ref)"))
  (`BlueprintGameplayTagLibrary.RemoveGameplayTag` (`self.EntityTags`) (struct :`TagName` "GameTags.Entity.Jumping"))
  (set `self.CurrentJumps` (`CharacterMovementComponent.MaxJumpApexAttemptsPerSimulation` (`self.CharacterMovement`))))

(fn `CheckCanMove`
  (if (`BlueprintGameplayTagLibrary.HasTag` (`self.EntityTags`) (struct :`TagName` "GameTags.Entity.Moveable"))
    (`self.EnableInput` (`GameplayStatics.GetPlayerController` 0) null)
    (else
      (`self.DisableInput` (`GameplayStatics.GetPlayerController` 0)))))

(fn `UserConstructionScript`)