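; AI controller for BP_Mech_Enemy that runs BT_MechEnemy and feeds its Blackboard.
; Perception of the player sets line of sight, target actor and TargetFound tag, with a DoOnce-gated timer around sight changes.
; It binds to the pawn's health damage events and has Alert and RemoveAlert events to set or clear the target.
; Tick latches IsDeadOrStaggered from entity tags and destroys the controller once the pawn is invalid.
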(event `self.ReceiveBeginPlay`
  (`self.RunBehaviorTree` "/Game/GameAssets/GameObjects/Characters/BT_MechEnemy.BT_MechEnemy")
  (bind _asbp_mech_enemy (cast `/Game/GameAssets/GameObjects/Characters/BP_Mech_Enemy` (`self.K2_GetPawn`)))
  (bind _output_get (set `self.SelfActor` _asbp_mech_enemy))
  (add `/Game/GameAssets/GameObjects/Components/BPC_Health.OnDamageTaken` (`/Game/GameAssets/GameObjects/Characters/BP_Mech_Base.BPC_Health` _output_get) (`|CreateDelegate` :!event `Alert`))
  (add `/Game/GameAssets/GameObjects/Components/BPC_Health.OnDamageTaken` (`/Game/GameAssets/GameObjects/Characters/BP_Mech_Base.BPC_Health` _output_get) (`|CreateDelegate` :!event `Alert`)))

(event `self.ReceiveTick`
  (params (DeltaSeconds :type "Float (single-precision)"))
  (bind _selfactor (`self.SelfActor`)
    (:`then`
      (bind _entitytags (`/Game/GameAssets/GameObjects/Characters/BP_Mech_Base.EntityTags` _selfactor))
      (if (or (`BlueprintGameplayTagLibrary.HasTag` _entitytags (struct :`TagName` "GameTags.Entity.Staggered")) (`BlueprintGameplayTagLibrary.HasTag` _entitytags (struct :`TagName` "GameTags.Entity.Dead")))
        (`BlackboardComponent.SetValueAsBool` (`self.Blackboard`) (`self.IsDeadOrStaggered`) true)))
    (:`else`
      (`self.K2_DestroyActor`))))

(event `self.AIPerception.OnTargetPerceptionUpdated`
  (params (Actor :type "Actor Object Reference") (Stimulus :type "AIStimulus Structure"))
  (bind _blackboard (`self.Blackboard`))
  (`self.SelfActor`
    (:`then`
      (if (and (`self.ActorHasTag` Actor "Player") (`.bSuccessfullySensed` (break `AIStimulus` Stimulus)))
        (`KismetSystemLibrary.K2_ClearAndInvalidateTimerHandle` (`self.EnemyTimer`))
        (`BlackboardComponent.SetValueAsBool` _blackboard (`self.HasLineOfSight`) true)
        (bind _asbp_mech_player (cast `/Game/GameAssets/GameObjects/Characters/BP_Mech_Player` (`GameplayStatics.GetPlayerCharacter` 0)))
        (`BlackboardComponent.SetValueAsObject` _blackboard (`self.EnemyActor`) _asbp_mech_player)
        (`BlueprintGameplayTagLibrary.AddGameplayTag` (`/Game/GameAssets/GameObjects/Characters/BP_Mech_Base.EntityTags` (`self.SelfActor`)) (struct :`TagName` "GameTags.Entity.TargetFound"))
        (`self.OnTargetSpotted`)
        (goto _label :!via `Reset`)
        (else
          (`/Engine/EditorBlueprintResources/StandardMacros.DoOnce` false :!label _label
            (:`Completed`
              (bind _returnvalue (`KismetSystemLibrary.K2_SetTimerDelegate` (`|CreateDelegate` :!event `StartEnemyTimer`) (`self.LineOfSightTimer`)))
              (set `self.EnemyTimer` _returnvalue))))))
    (:`else`
      (`self.K2_DestroyActor`))))

(event `StartEnemyTimer`
  (bind _blackboard (`self.Blackboard`))
  (`BlackboardComponent.SetValueAsBool` _blackboard (`self.HasLineOfSight`) true)
  (bind _asbp_mech_player (cast `/Game/GameAssets/GameObjects/Characters/BP_Mech_Player` (`GameplayStatics.GetPlayerPawn` 0)))
  (`BlackboardComponent.SetValueAsObject` _blackboard (`self.EnemyActor`) _asbp_mech_player)
  (`BlueprintGameplayTagLibrary.AddGameplayTag` (`/Game/GameAssets/GameObjects/Characters/BP_Mech_Base.EntityTags` (`self.SelfActor`)) (struct :`TagName` "GameTags.Entity.TargetFound"))
  (`self.OnTargetSpotted`))

(event `Alert`
  (bind _blackboard (`self.Blackboard`))
  (`BlackboardComponent.SetValueAsBool` _blackboard (`self.HasLineOfSight`) true)
  (`BlackboardComponent.SetValueAsObject` _blackboard (`self.EnemyActor`) (`GameplayStatics.GetPlayerPawn` 0))
  (`BlueprintGameplayTagLibrary.AddGameplayTag` (`/Game/GameAssets/GameObjects/Characters/BP_Mech_Base.EntityTags` (`self.SelfActor`)) (struct :`TagName` "GameTags.Entity.TargetFound"))
  (remove `/Game/GameAssets/GameObjects/Components/BPC_Health.OnDamageTaken` (`/Game/GameAssets/GameObjects/Characters/BP_Mech_Base.BPC_Health` (`self.SelfActor`)) (delegate `Alert`)))

(event `RemoveAlert`
  (bind _blackboard (`self.Blackboard`))
  (`BlackboardComponent.SetValueAsBool` _blackboard (`self.HasLineOfSight`) false)
  (`BlackboardComponent.SetValueAsObject` _blackboard (`self.EnemyActor`) null)
  (`BlueprintGameplayTagLibrary.RemoveGameplayTag` (`/Game/GameAssets/GameObjects/Characters/BP_Mech_Base.EntityTags` (`self.SelfActor`)) (struct :`TagName` "GameTags.Entity.TargetFound")))

(fn `UserConstructionScript`)