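; Player mech character that spawns two shoulder cannons and two machine guns on secondary and primary weapon platforms.
; Primary inputs fire the MGs, temporarily setting a firing tag, movement speed and shorter camera arm; secondary inputs are empty.
; A material parameter collection drives HUD parallax from smoothed camera rotation deltas, replaced by random shake while firing.
; It also handles camera switching, walking, HUD hit feedback and level reload after death.
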(event OnDamageTaken(BPC_Health)
  (bind _asbp_player_hud (Utilities|Casting|CastToBP_PlayerHUD (HUD|GetHUD (Game|GetPlayerController 0))))
  (Default|PlayHit _asbp_player_hud))

(event OnDeath(BPC_Health)
  (Development|PrintString "IM DEAD")
  (Utilities|FlowControl|Delay 3.0)
  (bind _returnvalue (Game|GetCurrentLevelName true))
  (Game|OpenLevel(byName) (Utilities|String|StringToName _returnvalue) false))

(event Custom|ResetFiring
  (GameplayTags|RemoveGameplayTag (Variables|Default|GetEntityTags) "(TagName=\"GameTags.Entity.FiringWeapon\")" :!class /Script/GameplayTags.BlueprintGameplayTagLibrary)
  (Variables|/Script/Engine.CharacterMovementComponent|SetMaxWalkSpeed (Variables|Character|GetCharacterMovement) (Utilities|Array|Get(acopy) (Variables|Default|GetMechSpeeds) 2))
  (Variables|/Script/Engine.SpringArmComponent|SetTargetArmLength (Variables|Default|GetSpringArm) 2.5e+02))

(event Input|EnhancedActionEvents|EnhancedInputActionIA_Primary_R
  (params (ActionValue :type Boolean) (ElapsedSeconds :type Float%20%28double-precision%29) (TriggeredSeconds :type Float%20%28double-precision%29) (InputAction :type Input%20Action%20Object%20Reference :default "/Game/GameAssets/Inputs/IA_Primary_R.IA_Primary_R"))
  (bind _weaponplatform_primary (Variables|Default|GetWeaponPlatform_Primary))
  (bind _weapon_r (Variables|/Game/GameAssets/GameObjects/Components/BPC_WeaponPlatform.BPC_WeaponPlatform_C|GetWeapon_R _weaponplatform_primary)
    (:then
      (bind _executed (Default|Fire _weaponplatform_primary _weapon_r))
      (if _executed
        (GameplayTags|AddGameplayTag (Variables|Default|GetEntityTags) "(TagName=\"GameTags.Entity.FiringWeapon\")" :!class /Script/GameplayTags.BlueprintGameplayTagLibrary)
        (Variables|/Script/Engine.CharacterMovementComponent|SetMaxWalkSpeed (Variables|Character|GetCharacterMovement) (Utilities|Array|Get(acopy) (Variables|Default|GetMechSpeeds) 1))
        (Variables|/Script/Engine.SpringArmComponent|SetTargetArmLength (Variables|Default|GetSpringArm) 1.5e+02)
        (Utilities|Time|SetTimerbyEvent (delegate Custom|ResetFiring) 0.5)))
    (:else)))

(event Input|EnhancedActionEvents|EnhancedInputActionIA_Primary_L
  (params (ActionValue :type Boolean) (ElapsedSeconds :type Float%20%28double-precision%29) (TriggeredSeconds :type Float%20%28double-precision%29) (InputAction :type Input%20Action%20Object%20Reference :default "/Game/GameAssets/Inputs/IA_Primary_L.IA_Primary_L"))
  (bind _weaponplatform_primary (Variables|Default|GetWeaponPlatform_Primary))
  (bind _weaponplatform_primary_2 (Variables|Default|GetWeaponPlatform_Primary))
  (bind _weapon_l (Variables|/Game/GameAssets/GameObjects/Components/BPC_WeaponPlatform.BPC_WeaponPlatform_C|GetWeapon_L _weaponplatform_primary_2)
    (:then
      (bind _executed (Default|Fire _weaponplatform_primary_2 _weapon_l))
      (if _executed
        (GameplayTags|AddGameplayTag (Variables|Default|GetEntityTags) "(TagName=\"GameTags.Entity.FiringWeapon\")" :!class /Script/GameplayTags.BlueprintGameplayTagLibrary :!label _label)
        (Variables|/Script/Engine.CharacterMovementComponent|SetMaxWalkSpeed (Variables|Character|GetCharacterMovement) (Utilities|Array|Get(acopy) (Variables|Default|GetMechSpeeds) 1))
        (Variables|/Script/Engine.SpringArmComponent|SetTargetArmLength (Variables|Default|GetSpringArm) 1.5e+02)
        (Utilities|Time|SetTimerbyEvent (delegate Custom|ResetFiring) 0.5)
        (else
          (bind _weapon_r (Variables|/Game/GameAssets/GameObjects/Components/BPC_WeaponPlatform.BPC_WeaponPlatform_C|GetWeapon_R _weaponplatform_primary)
            (:then
              (bind _executed_2 (Default|Fire _weaponplatform_primary _weapon_r))
              (if _executed_2
                (goto _label)))
            (:else)))))
    (:else)))

(event Input|EnhancedActionEvents|EnhancedInputActionIA_Secondary_R
  (params (ActionValue :type Boolean) (ElapsedSeconds :type Float%20%28double-precision%29) (TriggeredSeconds :type Float%20%28double-precision%29) (InputAction :type Input%20Action%20Object%20Reference :default "/Game/GameAssets/Inputs/IA_Secondary_R.IA_Secondary_R")))

(event Input|EnhancedActionEvents|EnhancedInputActionIA_CameraSwitch
  (params (ActionValue :type Boolean) (ElapsedSeconds :type Float%20%28double-precision%29) (TriggeredSeconds :type Float%20%28double-precision%29) (InputAction :type Input%20Action%20Object%20Reference :default "/Game/GameAssets/Inputs/IA_CameraSwitch.IA_CameraSwitch"))
  (Utilities|FlowControl|FlipFlop
    (:A
      (Components|Activation|SetActive (Variables|Default|GetCamera) false false)
      (Variables|Default|SetActiveCamera (Variables|Default|GetTPS_Camera)))
    (:B
      (Components|Activation|SetActive (Variables|Default|GetCamera) true false)
      (Variables|Default|SetActiveCamera (Variables|Default|GetCamera)))))

(event Input|EnhancedActionEvents|EnhancedInputActionIA_Walk
  (params (ActionValue :type Boolean) (ElapsedSeconds :type Float%20%28double-precision%29) (TriggeredSeconds :type Float%20%28double-precision%29) (InputAction :type Input%20Action%20Object%20Reference :default "/Game/GameAssets/Inputs/IA_Walk.IA_Walk"))
  (:Triggered
    (Variables|/Script/Engine.CharacterMovementComponent|SetMaxWalkSpeed (Variables|Character|GetCharacterMovement) 6e+02))
  (:Canceled
    (Variables|/Script/Engine.CharacterMovementComponent|SetMaxWalkSpeed (Variables|Character|GetCharacterMovement) 1e+03 :!label _label))
  (:Completed
    (goto _label)))

(event Input|EnhancedActionEvents|EnhancedInputActionIA_Secondary_L
  (params (ActionValue :type Boolean) (ElapsedSeconds :type Float%20%28double-precision%29) (TriggeredSeconds :type Float%20%28double-precision%29) (InputAction :type Input%20Action%20Object%20Reference :default "/Game/GameAssets/Inputs/IA_Secondary_L.IA_Secondary_L")))

(event EventBeginPlay
  (|CallParentFunction)
  (for _index (range 0 1)
    (bind _returnvalue (Game|SpawnActorfromClass "/Game/GameAssets/GameObjects/Weapons/BP_ShoulderCannon.BP_ShoulderCannon_C" (Transformation|GetActorTransform) "Undefined" "MultiplyWithRoot" self 0))
    (Default|AddWeapon (Variables|Default|GetWeaponPlatform_Secondary) _returnvalue))
  (for _index_2 (range 0 1)
    (bind _returnvalue_2 (Game|SpawnActorfromClass "/Game/GameAssets/GameObjects/Weapons/BP_MG.BP_MG_C" (Transformation|GetActorTransform) "Undefined" "MultiplyWithRoot" self 0))
    (Default|AddWeapon (Variables|Default|GetWeaponPlatform_Primary) _returnvalue_2)))

(event Collision|EventActorBeginOverlap
  (params (OtherActor :type Actor%20Object%20Reference))
  (|CallParentFunction OtherActor) ; This node is disabled and will not be called.\nDrag off pins to build functionality.
)

(event EventTick
  (params (DeltaSeconds :type Float%20%28single-precision%29))
  (|CallParentFunction DeltaSeconds)
  (if (GameplayTags|HasTag (Variables|Default|GetEntityTags) "(TagName=\"GameTags.Entity.FiringWeapon\")")
    (Rendering|Material|SetVectorParameterValue "/Game/GameAssets/GameObjects/Visuals/PlayerHUD/MPC_Parallax.MPC_Parallax" "ParallaxOffset" (Utilities|Struct|MakeLinearColor (Math|Random|RandomFloatinRange -2.5 2.5) (Math|Random|RandomFloatinRange -2.5 2.5) 0.0 1.0) :!class /Script/Engine.KismetMaterialLibrary)
    (else
      (CallFunction|CalculateParallaxHUD))))

(event Input|KeyboardEvents|DebugKeyJ
  (params (Key :type Key%20Structure :default "None") (ActionValue :type Input%20Action%20Value%20Structure))
  (:Pressed
    (Default|TakeDamage (Variables|Default|GetBPC_Health) 5.0)))

(fn ConstructionScript
  (|CallParentFunction))

(fn CalculateParallaxHUD
  (bind _activecamera (Variables|Default|GetActiveCamera))
  (bind _minmaxpitchrate (Variables|Default|GetMinMaxPitchRate))
  (bind _minmaxyawrate (Variables|Default|GetMinMaxYawRate))
  (bind _returnvalue (Transformation|GetWorldRotation _activecamera))
  (bind (_roll _pitch _yaw) (Math|Rotator|BreakRotator _returnvalue))
  (Variables|Default|SetPitchRate (Math|Float|Clamp(Float) (+ (Variables|Default|GetPitchRate) (- _pitch (.pitch (Variables|Default|GetCameraRot)))) (* _minmaxpitchrate -1.0) _minmaxpitchrate))
  (Variables|Default|SetYawRate (Math|Float|Clamp(Float) (+ (Variables|Default|GetYawRate) (- _yaw (.yaw (Variables|Default|GetCameraRot)))) (* _minmaxyawrate -1.0) _minmaxyawrate))
  (Variables|Default|SetCameraRot (Transformation|GetWorldRotation (Variables|Default|GetActiveCamera)))
  (Variables|Default|SetPitch%20Parallax%20Offset (Math|Interpolation|FInterpTo (Variables|Default|GetPitch%20Parallax%20Offset) (Variables|Default|GetPitchRate) (Utilities|Time|GetWorldDeltaSeconds) 5.0))
  (Variables|Default|SetYaw%20Parallax%20Offset (Math|Interpolation|FInterpTo (Variables|Default|GetYaw%20Parallax%20Offset) (Variables|Default|GetYawRate) (Utilities|Time|GetWorldDeltaSeconds) 5.0))
  (Rendering|Material|SetVectorParameterValue "/Game/GameAssets/GameObjects/Visuals/PlayerHUD/MPC_Parallax.MPC_Parallax" "ParallaxOffset" (Utilities|Struct|MakeLinearColor (Variables|Default|GetYaw%20Parallax%20Offset) (Variables|Default|GetPitch%20Parallax%20Offset) 0.0 1.0) :!class /Script/Engine.KismetMaterialLibrary))