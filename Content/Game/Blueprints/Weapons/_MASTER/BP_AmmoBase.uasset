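; BP_AmmoBase is a base projectile actor for weapon ammo, configured by an AmmoData variable.
; The construction script applies its speed, lifespan and hit radius to the projectile movement, actor and collision sphere.
; On overlap, it looks up a HealthComponent on the other actor, applies the data's damage and destroys itself.
; Without that component it only prints an error and persists; debug prints report hits and health.
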(event `self.ReceiveActorBeginOverlap`
  (params (OtherActor :type "Actor Object Reference"))
  (bind _returnvalue (`self.GetComponentByClass` OtherActor "/Game/Game/Blueprints/ActorComponents/HealthComponent.HealthComponent_C"))
  (bind (_ammodata_lifespan _ammodata_speed _ammodata_hitradius _ammodata_damage) (break `/Game/Game/Blueprints/Weapons/_MASTER/St_AmmoStruct` (`self.AmmoData`)))
  (`KismetSystemLibrary.PrintString` "BEGUN HIT")
  (`/Engine/EditorBlueprintResources/StandardMacros.IsValid` _returnvalue
    (:`Is Valid`
      (`/Game/Game/Blueprints/ActorComponents/HealthComponent.TakeDamage` _returnvalue _ammodata_damage)
      (`KismetSystemLibrary.PrintString` (`KismetStringLibrary.Conv_DoubleToString` (`/Game/Game/Blueprints/ActorComponents/HealthComponent.Health` _returnvalue)))
      (`self.K2_DestroyActor`))
    (:`Is Not Valid`
      (`KismetSystemLibrary.PrintString` "ERROR: FAILED TO FIND COMPONENT / TAKE DAMAGE"))))

(fn `UserConstructionScript`
  (bind _projectilemovement (`self.ProjectileMovement`))
  (bind (_ammodata_lifespan _ammodata_speed _ammodata_hitradius) (break `/Game/Game/Blueprints/Weapons/_MASTER/St_AmmoStruct` (`self.AmmoData`)))
  (set `ProjectileMovementComponent.InitialSpeed` _ammodata_speed _projectilemovement)
  (set `ProjectileMovementComponent.MaxSpeed` _ammodata_speed _projectilemovement)
  (`self.SetLifeSpan` _ammodata_lifespan)
  (`SphereComponent.SetSphereRadius` (`self.Sphere`) _ammodata_hitradius true))