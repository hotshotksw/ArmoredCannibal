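; BP_WeaponBase is a master weapon Blueprint that handles firing, ammo use and depletion.
; Fire requires a valid Ammo class, plays a pitch-randomized sound, then either runs a hitscan or spawns a projectile, returning the fire rate.
; Hitscan sphere-traces from the owner's camera with debug drawing and damages HealthComponents.
; UseAmmo deducts shot cost unless infinite; OnWeaponDestroyed fires on empty reserve or failed spawn.
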(fn `Fire`
  (returns (Firerate :type "Float (double-precision)"))
  (bind _ammo (`self.Ammo`))
  (bind (_weapondata_type _weapondata_position _weapondata_firerate _weapondata_ishitscan _weapondata_infiniteammo) (break `/Game/Game/Blueprints/Weapons/_MASTER/St_WeaponStruct` (`self.WeaponData`)))
  (bind _staticmesh (`self.StaticMesh`))
  (if (`KismetSystemLibrary.IsValidClass` _ammo)
    (`GameplayStatics.PlaySoundAtLocation` "/Game/Game/Audio/machinegun.machinegun" (`SceneComponent.K2_GetComponentLocation` _staticmesh) (`SceneComponent.K2_GetComponentRotation` _staticmesh) 0.25 (`KismetMathLibrary.RandomFloatInRange` 0.85 1.15) 0.0 "/Game/Game/Audio/SA_Gun.SA_Gun" null null null)
    (if _weapondata_ishitscan
      (bind _cost (`self.FireHitscan`))
      (`self.UseAmmo` _weapondata_infiniteammo _cost)
      (return _weapondata_firerate)
      (else
        (bind _returnvalue (`|SpawnActorFromClass` _ammo (`SceneComponent.K2_GetComponentToWorld` (`self.BarrelArrow`)) "Undefined" "OverrideRootScale" null (`self.WeaponOwner`) null))
        (`/Engine/EditorBlueprintResources/StandardMacros.IsValid` _returnvalue
          (:`Is Valid`
            (bind (_ammodata_lifespan _ammodata_speed _ammodata_hitradius _ammodata_damage _ammodata_cost) (break `/Game/Game/Blueprints/Weapons/_MASTER/St_AmmoStruct` (`/Game/Game/Blueprints/Weapons/_MASTER/BP_AmmoBase.AmmoData` _returnvalue)))
            (`self.UseAmmo` _weapondata_infiniteammo _ammodata_cost)
            (return _weapondata_firerate))
          (:`Is Not Valid`
            (`self.OnWeaponDestroyed`)))))
    (else
      (return 0.0))))

(fn `FireHitscan`
  (returns (Cost :type Integer))
  (bind (_hitscandata_range _hitscandata_damage _hitscandata_cost) (break `/Game/Game/Blueprints/Weapons/_MASTER/St_HitscanStruct` (`self.HitscanData`)))
  (bind _hitscandata_range_2 (break `/Game/Game/Blueprints/Weapons/_MASTER/St_HitscanStruct` (`self.HitscanData`)))
  (bind _camera (`/Game/Game/Blueprints/Characters/Master/BP_CharacterBase.Camera` (`self.WeaponOwner`)))
  (bind _returnvalue (`SceneComponent.K2_GetComponentLocation` _camera))
  (bind _outhit (`KismetSystemLibrary.SphereTraceSingleForObjects` _returnvalue (+ _returnvalue (* (`KismetMathLibrary.GetForwardVector` (`SceneComponent.K2_GetComponentRotation` _camera)) _hitscandata_range_2)) 4.0 (`|MakeArray` "ObjectTypeQuery1" "ObjectTypeQuery3" :!type "EObjectTypeQuery Enum") false (`|MakeArray` (`self.WeaponOwner`) :!type "Actor Object Reference") "ForDuration" true (struct :`R` 1.0 :`A` 1.0) (struct :`G` 1.0 :`A` 1.0) 1.0))
  (`/Engine/EditorBlueprintResources/StandardMacros.IsValid` (`.HitActor` (`GameplayStatics.BreakHitResult` _outhit))
    (:`Is Valid`
      (bind _returnvalue_2 (`self.GetComponentByClass` (`.HitActor` (`GameplayStatics.BreakHitResult` _outhit)) "/Game/Game/Blueprints/ActorComponents/HealthComponent.HealthComponent_C"))
      (`/Engine/EditorBlueprintResources/StandardMacros.IsValid` _returnvalue_2
        (:`Is Valid`
          (`/Game/Game/Blueprints/ActorComponents/HealthComponent.TakeDamage` _returnvalue_2 _hitscandata_damage))
        (:`Is Not Valid`
          (`KismetSystemLibrary.PrintString` "ERROR: FAILED TO FIND COMPONENT / TAKE DAMAGE")))
      (return _hitscandata_cost))
    (:`Is Not Valid`
      (return _hitscandata_cost))))

(fn `UseAmmo`
  (params (HasInfiniteAmmo :type Boolean) (Cost :type Integer))
  (if (not HasInfiniteAmmo)
    (bind _output_get (set `self.AmmoReserve` (- (`self.AmmoReserve`) Cost)))
    (`KismetSystemLibrary.PrintString` (`KismetStringLibrary.Conv_IntToString` _output_get))
    (if (<= _output_get 0)
      (`self.OnWeaponDestroyed`))))

(fn `UserConstructionScript`)