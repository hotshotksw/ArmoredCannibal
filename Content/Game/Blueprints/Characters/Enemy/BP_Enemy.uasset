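; Enemy character that runs the BT_Enemy behavior tree, targets the player and carries infinite-ammo machine guns.
; HealthComponent supplies the health bar and drives damage and death events.
; At about a third health it gains the Staggered gameplay tag and an execute component with an attached sphere.
; Death plays a crash sound, disables collision, destroys weapons, tags it Dead and starts a five-second timer.
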(event `self.ReceiveBeginPlay`
  (bind _healthcomponent (`self.HealthComponent`))
  (`AIController.RunBehaviorTree` (`AIBlueprintHelperLibrary.GetAIController` self) "/Game/Game/Blueprints/Characters/Enemy/BT_Enemy.BT_Enemy")
  (`parent.ReceiveBeginPlay`)
  (`/Game/Game/Blueprints/ActorComponents/HealthComponent.CreateEnemyHealthbar` (`self.HealthComponent`))
  (add `/Game/Game/Blueprints/ActorComponents/HealthComponent.OnDamageTaken` _healthcomponent (delegate `OnDamageTaken_Event`))
  (add `/Game/Game/Blueprints/ActorComponents/HealthComponent.OnDeath` _healthcomponent (delegate `OnDeath_Event`))
  (bind (_socketname _weapon) (`self.AttachWeapon` "/Game/Game/Blueprints/Weapons/MachineGun/BP_MachineGun.BP_MachineGun_C"))
  (`/Game/Game/Blueprints/ActorComponents/WeaponComponent.SetInfiniteAmmo` _weapon)
  (bind (_socketname_2 _weapon_2) (`self.AttachWeapon` "/Game/Game/Blueprints/Weapons/MachineGun/BP_MachineGun.BP_MachineGun_C"))
  (`/Game/Game/Blueprints/ActorComponents/WeaponComponent.SetInfiniteAmmo` _weapon_2)
  (`SceneComponent.K2_AttachToComponent` (`self.Camera`) (`self.Mesh`) "B_HeadSocket" "SnapToTarget" "SnapToTarget" "KeepRelative" true)
  (bind _asbp_player (cast `/Game/Game/Blueprints/Characters/Master/BP_Player` (`GameplayStatics.GetPlayerCharacter` 0)))
  (set `self.Target` _asbp_player))

(event `OnDamageTaken_Event`
  (bind _healthcomponent (`self.HealthComponent`))
  (if (<= (/ (`/Game/Game/Blueprints/ActorComponents/HealthComponent.Health` _healthcomponent) (`/Game/Game/Blueprints/ActorComponents/HealthComponent.MaxHealth` _healthcomponent)) 0.334)
    (`/Engine/EditorBlueprintResources/StandardMacros.DoOnce` false
      (:`Completed`
        (`BlueprintGameplayTagLibrary.AddGameplayTag` (`self.CharacterTags`) (struct :`TagName` "CharacterStatus.Staggered"))
        (bind _returnvalue (`AddComponent|NODE_AddExecuteComponent-3`))
        (`/Game/Game/Blueprints/ActorComponents/ExecuteComponent.AttachExecuteSphere` _returnvalue self)
        (`KismetSystemLibrary.PrintString` "YOU GONNA DIE" true true (struct :`G` 0.66 :`B` 1.0 :`A` 1.0) 0.1)))))

(event `OnDeath_Event`
  (params (DeadCharacter :type "/Game/Game/Blueprints/Characters/Master/BP_CharacterBase Object Reference"))
  (`/Engine/EditorBlueprintResources/StandardMacros.DoOnce` false
    (:`Completed`
      (`GameplayStatics.PlaySoundAtLocation` "/Game/Game/Audio/crash.crash" (`SceneComponent.K2_GetComponentLocation` (`self.CapsuleComponent`)) (struct) 1.0 1.0 0.0 "/Game/Game/Audio/SA_Gun.SA_Gun" null null null)
      (`self.KillEnemy`))))

(event `Destroy`
  (`self.K2_DestroyActor`))

(event `self.ReceiveActorBeginOverlap`
  (params (OtherActor :type "Actor Object Reference")))

(fn `KillEnemy`
  (bind _primaryleft (`self.PrimaryLeft`))
  (bind _primaryright (`self.PrimaryRight`))
  (bind _primaryleft_2 (`self.PrimaryLeft`))
  (bind _secondaryright (`self.SecondaryRight`))
  (bind _secondaryleft (`self.SecondaryLeft`))
  (`|ExecutionSequence`
    (:`then_1`
      (`self.SetActorEnableCollision` false)
      (`Widget.SetVisibility` (`/Game/Game/Blueprints/ActorComponents/HealthComponent.EnemyHealthBar` (`self.HealthComponent`)) "Hidden")
      (`BlueprintGameplayTagLibrary.RemoveGameplayTag` (`self.CharacterTags`) (struct :`TagName` "CharacterStatus.TargetFound")))
    (:`then_2`
      (`/Engine/EditorBlueprintResources/StandardMacros.IsValid` _primaryleft
        (:`Is Valid`
          (`self.AttachWeapon` (`GameplayStatics.GetObjectClass` (`/Game/Game/Blueprints/ActorComponents/WeaponComponent.Weapon` _primaryleft))))))
    (:`then_3`
      (`/Engine/EditorBlueprintResources/StandardMacros.IsValid` _primaryright
        (:`Is Valid`
          (`/Game/Game/Blueprints/ActorComponents/WeaponComponent.DestroyWeapon` _primaryright))))
    (:`then_4`
      (`/Engine/EditorBlueprintResources/StandardMacros.IsValid` _primaryleft_2
        (:`Is Valid`
          (`/Game/Game/Blueprints/ActorComponents/WeaponComponent.DestroyWeapon` _primaryleft_2))))
    (:`then_5`
      (`/Engine/EditorBlueprintResources/StandardMacros.IsValid` _secondaryright
        (:`Is Valid`
          (`/Game/Game/Blueprints/ActorComponents/WeaponComponent.DestroyWeapon` _secondaryright))))
    (:`then_6`
      (`/Engine/EditorBlueprintResources/StandardMacros.IsValid` _secondaryleft
        (:`Is Valid`
          (`/Game/Game/Blueprints/ActorComponents/WeaponComponent.DestroyWeapon` _secondaryleft))))
    (:`then_7`
      (`PrimitiveComponent.SetCollisionEnabled` (`self.CapsuleComponent`) "NoCollision")
      (`BlueprintGameplayTagLibrary.AddGameplayTag` (`self.CharacterTags`) (struct :`TagName` "CharacterStatus.Dead"))
      (`KismetSystemLibrary.K2_SetTimerDelegate` (`|CreateDelegate` :!event `Destroy`) 5.0))))

(fn `UserConstructionScript`
  (`parent.UserConstructionScript`))