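; Base character Blueprint providing four weapon slots, crouching and jump-count reset on landing.
; AttachWeapon fills free primary (right first) or secondary (left first) slots with new weapon components on mesh sockets.
; Fire events call each slot's component; primary-left also plays a montage, or falls back to primary-right when empty.
; Crouch removes ground friction, raises gravity and shrinks the capsule via a Timeline, which reverses on release.
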(event `FireSecondaryLeft`
  (bind _secondaryleft (`self.SecondaryLeft`))
  (`/Engine/EditorBlueprintResources/StandardMacros.IsValid` _secondaryleft
    (:`Is Valid`
      (`/Game/Game/Blueprints/ActorComponents/WeaponComponent.FireWeapon` _secondaryleft))))

(event `FireSecondaryRight`
  (bind _secondaryright (`self.SecondaryRight`))
  (`/Engine/EditorBlueprintResources/StandardMacros.IsValid` _secondaryright
    (:`Is Valid`
      (`/Game/Game/Blueprints/ActorComponents/WeaponComponent.FireWeapon` _secondaryright))))

(event `FirePrimaryRight`
  (bind _primaryright (`self.PrimaryRight`))
  (`/Engine/EditorBlueprintResources/StandardMacros.IsValid` _primaryright :!label _label
    (:`Is Valid`
      (`/Game/Game/Blueprints/ActorComponents/WeaponComponent.FireWeapon` _primaryright))))

(event `FirePrimaryLeft`
  (bind _primaryleft (`self.PrimaryLeft`))
  (`/Engine/EditorBlueprintResources/StandardMacros.IsValid` _primaryleft
    (:`Is Valid`
      (`self.UseAnimation`)
      (`/Game/Game/Blueprints/ActorComponents/WeaponComponent.FireWeapon` _primaryleft))
    (:`Is Not Valid`
      (goto _label))))

(event `self.OnLanded`
  (params (Hit :type "HitResult Structure (by ref)"))
  (bind _output_get (set `self.CurrentJumps` (`CharacterMovementComponent.MaxJumpApexAttemptsPerSimulation` (`self.CharacterMovement`))))
  (`KismetSystemLibrary.PrintString` (`KismetStringLibrary.Concat_StrStr` "Jumps Remaining: " (`KismetStringLibrary.Conv_IntToString` _output_get))))

(event `CharacterCrouch`
  (bind _charactermovement (`self.CharacterMovement`))
  (set `self.IsCrouched` true)
  (if (!= (`CharacterMovementComponent.GroundFriction` _charactermovement) 0.4)
    (set `CharacterMovementComponent.GroundFriction` 0.0 _charactermovement)
    (set `CharacterMovementComponent.GravityScale` 4.0 _charactermovement)
    (bind (_direction _crouchtime) (`Timeline|Timeline` :!label _label_2)
      (:`Update`
        (`CapsuleComponent.SetCapsuleHalfHeight` (`self.CapsuleComponent`) (`KismetMathLibrary.Lerp` 110.0 25.0 _crouchtime) true)))))

(event `CharacterStopCrouch`
  (bind _charactermovement (`self.CharacterMovement`))
  (set `self.IsCrouched` false)
  (set `CharacterMovementComponent.GroundFriction` 8.0 _charactermovement)
  (set `CharacterMovementComponent.GravityScale` 2.0 _charactermovement)
  (goto _label_2 :!via `Reverse`))

(fn `AttachWeapon`
  (params (NewWeapon :type "/Game/Game/Blueprints/Weapons/_MASTER/BP_WeaponBase Class Reference") (WeaponPosition :type "/Game/Game/Blueprints/Weapons/_MASTER/E_WeaponPosition Enum" :default "NewEnumerator0"))
  (bind _mesh (`self.Mesh`))
  (bind _mesh_2 (`self.Mesh`))
  (if (`|EnumEquality` WeaponPosition "NewEnumerator0")
    ;[0.1927 0 0] Primary Weapon Addition
    (`/Engine/EditorBlueprintResources/StandardMacros.IsValid` (`self.PrimaryRight`)
      (:`Is Valid`
        (`/Engine/EditorBlueprintResources/StandardMacros.IsValid` (`self.PrimaryLeft`)
          (:`Is Not Valid`
            (bind _returnvalue (`AddComponent|NODE_AddWeaponComponent-0`))
            (bind _output_get (set `self.PrimaryLeft` _returnvalue))
            (`/Game/Game/Blueprints/ActorComponents/WeaponComponent.AttachWeaponToSocket` _output_get NewWeapon (`SceneComponent.GetSocketTransform` _mesh_2 "P_WeaponLeft" "RTS_World") "P_WeaponLeft" self))))
      (:`Is Not Valid`
        (bind _returnvalue_2 (`AddComponent|NODE_AddWeaponComponent-1`))
        (bind _output_get_2 (set `self.PrimaryRight` _returnvalue_2))
        (`/Game/Game/Blueprints/ActorComponents/WeaponComponent.AttachWeaponToSocket` _output_get_2 NewWeapon (`SceneComponent.GetSocketTransform` _mesh_2 "P_WeaponRight" "RTS_World") "P_WeaponRight" self)))
    (else
      ;[0.03049 0.01628 0.1562] Secondary Weapon Addition
      (`/Engine/EditorBlueprintResources/StandardMacros.IsValid` (`self.SecondaryLeft`)
        (:`Is Valid`
          (`/Engine/EditorBlueprintResources/StandardMacros.IsValid` (`self.SecondaryRight`)
            (:`Is Not Valid`
              (bind _returnvalue_3 (`AddComponent|NODE_AddWeaponComponent-2`))
              (bind _output_get_3 (set `self.SecondaryRight` _returnvalue_3))
              (`/Game/Game/Blueprints/ActorComponents/WeaponComponent.AttachWeaponToSocket` _output_get_3 NewWeapon (`SceneComponent.GetSocketTransform` _mesh "S_WeaponRight" "RTS_World") "S_WeaponRight" self))))
        (:`Is Not Valid`
          (bind _returnvalue_4 (`AddComponent|NODE_AddWeaponComponent-3`))
          (bind _output_get_4 (set `self.SecondaryLeft` _returnvalue_4))
          (`/Game/Game/Blueprints/ActorComponents/WeaponComponent.AttachWeaponToSocket` _output_get_4 NewWeapon (`SceneComponent.GetSocketTransform` _mesh "S_WeaponLeft" "RTS_World") "S_WeaponLeft" self))))))

(fn `UseAnimation`
  (bind _animmontage (`self.AnimMontage`))
  (`/Engine/EditorBlueprintResources/StandardMacros.IsValid` _animmontage
    (:`Is Valid`
      (`self.PlayAnimMontage` _animmontage))))

(fn `UserConstructionScript`)