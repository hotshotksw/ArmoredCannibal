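; Player character Blueprint that maps Enhanced Input to look, movement, crouch, four weapon slots and a two-stage jump with a launched boost.
; Gameplay tags gate actions through CanMove and track jumping, while parent class functions handle weapon attachment.
; Death from HealthComponent triggers physics, removes CanMove and shows the game-over widget once.
; It also fades the HUD and health bar, refreshes ammo widgets and has debug keys for weapons, invincibility and self-kill.
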(event Custom|PlayerDeath
  (params (DeadCharacter :type BP%20Character%20Base%20Object%20Reference))
  (Utilities|FlowControl|DoOnce false
    (:Completed
      (Audio|PlaySound2D "/Game/GameAssets/Audio/crash.crash" 1.0 1.0 0.0 0 0)
      (Physics|SetSimulatePhysics (Variables|Default|GetCapsuleComponent) true)
      (GameplayTags|RemoveGameplayTag (Variables|Default|GetCharacterTags) "(TagName=\"CharacterStatus.CanMove\")" :!class /Script/GameplayTags.BlueprintGameplayTagLibrary)
      (bind _returnvalue (UserInterface|CreateWidget "/Game/Game/Blueprints/Visual/GameOver/W_GameOver.W_GameOver_C"))
      (UserInterface|Viewport|AddtoViewport _returnvalue 0))))

(event Input|EnhancedActionEvents|EnhancedInputActionIA_Execute
  (params (ActionValue :type Boolean) (ElapsedSeconds :type Float%20%28double-precision%29) (TriggeredSeconds :type Float%20%28double-precision%29) (InputAction :type Input%20Action%20Object%20Reference :default "/Game/Game/Inputs/Execute/IA_Execute.IA_Execute"))
  (Default|CallOnExecuting))

(event EventBeginPlay
  (|CallParentFunction)
  (EventDispatchers|BindEventtoOnDeath (Variables|Default|GetHealthComponent) (EventDispatchers|CreateEvent :!event Custom|PlayerDeath)))

(event Collision|EventActorBeginOverlap
  (params (OtherActor :type Actor%20Object%20Reference))
  (|CallParentFunction OtherActor))

(event EventTick
  (params (DeltaSeconds :type Float%20%28single-precision%29)))

(event Input|KeyboardEvents|DebugKeyBackspace
  (params (Key :type Key%20Structure :default "None") (ActionValue :type Input%20Action%20Value%20Structure))
  (:Pressed
    (Transformation|AttachComponentToComponent (Variables|Default|GetCamera) (Variables|Character|GetMesh) "B_Head" "KeepWorld" "KeepRelative" "KeepRelative" true)
    (Default|TakeDamage (Variables|Default|GetHealthComponent) 1e+03)))

(fn ConstructionScript
  (|CallParentFunction))

(fn UpdateAmmo
  (bind _foundwidgets (Widget|GetAllWidgetsOfClass "/Game/Game/Blueprints/Visual/PlayerHUD/W_WeaponList.W_WeaponList_C" false))
  (if (> (Utilities|Array|Length _foundwidgets) 0)
    (for _array_element _foundwidgets
      (Default|UpdateAmmo _array_element))))

(fn AttachWeapon
  (params (NewWeapon :type BP%20Weapon%20Base%20Class%20Reference) (WeaponPosition :type E_WeaponPosition%20Enum :default "NewEnumerator0") (HasInfiniteAmmo :type Boolean))
  (|CallParentFunction NewWeapon WeaponPosition HasInfiniteAmmo))

(fn TransitionHUD
  (bind _playerhud (Variables|Default|GetPlayerHUD)
    (:then
      (if (Variables|/Game/Game/Blueprints/Visual/PlayerHUD/W_PlayerHUD.W_PlayerHUD_C|GetActivated _playerhud)
        (UserInterface|Animation|PlayAnimation (Variables|Default|GetPlayerHUD) (Variables|/Game/Game/Blueprints/Visual/PlayerHUD/W_PlayerHUD.W_PlayerHUD_C|GetFade (Variables|Default|GetPlayerHUD)) 0.0 1 "Reverse" 1.0 false)
        (else
          (UserInterface|Animation|PlayAnimation (Variables|Default|GetPlayerHUD) (Variables|/Game/Game/Blueprints/Visual/PlayerHUD/W_PlayerHUD.W_PlayerHUD_C|GetFade (Variables|Default|GetPlayerHUD)) 0.0 1 "Forward" 1.0 false))))
    (:else
      (bind _returnvalue (UserInterface|CreateWidget "/Game/Game/Blueprints/Visual/PlayerHUD/W_PlayerHUD.W_PlayerHUD_C"))
      (bind _output_get (Variables|Default|SetPlayerHUD _returnvalue))
      (UserInterface|Viewport|AddtoViewport _output_get 0)
      (UserInterface|Animation|PlayAnimation _output_get (Variables|/Game/Game/Blueprints/Visual/PlayerHUD/W_PlayerHUD.W_PlayerHUD_C|GetFade _output_get) 0.0 1 "Forward" 1.0 false)))
  (bind _healthcomponent (Variables|Default|GetHealthComponent)
    (:then
      (bind _playerhealthbar (Variables|/Game/Game/Blueprints/ActorComponents/HealthComponent.HealthComponent_C|GetPlayerHealthBar _healthcomponent)
        (:then
          _)
        (:else
          (Default|CreatePlayerHealthbar _healthcomponent)))
      (if (Variables|/Game/Game/Blueprints/Visual/PlayerHUD/W_PlayerHealth.W_PlayerHealth_C|GetActivated _playerhealthbar)
        (UserInterface|Animation|PlayAnimation (Variables|/Game/Game/Blueprints/ActorComponents/HealthComponent.HealthComponent_C|GetPlayerHealthBar _healthcomponent) (Variables|/Game/Game/Blueprints/Visual/PlayerHUD/W_PlayerHealth.W_PlayerHealth_C|GetFade (Variables|/Game/Game/Blueprints/ActorComponents/HealthComponent.HealthComponent_C|GetPlayerHealthBar _healthcomponent)) 0.0 1 "Reverse" 1.0 false)
        (else
          (UserInterface|Animation|PlayAnimation (Variables|/Game/Game/Blueprints/ActorComponents/HealthComponent.HealthComponent_C|GetPlayerHealthBar _healthcomponent) (Variables|/Game/Game/Blueprints/Visual/PlayerHUD/W_PlayerHealth.W_PlayerHealth_C|GetFade (Variables|/Game/Game/Blueprints/ActorComponents/HealthComponent.HealthComponent_C|GetPlayerHealthBar _healthcomponent)) 0.0 1 "Forward" 1.0 false))))
    (:else)))

(event Input|EnhancedActionEvents|EnhancedInputActionIA_PrimaryLeft
  (params (ActionValue :type Boolean) (ElapsedSeconds :type Float%20%28double-precision%29) (TriggeredSeconds :type Float%20%28double-precision%29) (InputAction :type Input%20Action%20Object%20Reference :default "/Game/Game/Inputs/Weapons/IA_PrimaryLeft.IA_PrimaryLeft"))
  (if (GameplayTags|HasTag (Variables|Default|GetCharacterTags) "(TagName=\"CharacterStatus.CanMove\")")
    (CallFunction|FirePrimaryLeft)))

(event Input|EnhancedActionEvents|EnhancedInputActionIA_PrimaryRight
  (params (ActionValue :type Boolean) (ElapsedSeconds :type Float%20%28double-precision%29) (TriggeredSeconds :type Float%20%28double-precision%29) (InputAction :type Input%20Action%20Object%20Reference :default "/Game/Game/Inputs/Weapons/IA_PrimaryRight.IA_PrimaryRight"))
  (if (GameplayTags|HasTag (Variables|Default|GetCharacterTags) "(TagName=\"CharacterStatus.CanMove\")")
    (CallFunction|FirePrimaryRight)))

(event Input|EnhancedActionEvents|EnhancedInputActionIA_SecondaryLeft
  (params (ActionValue :type Boolean) (ElapsedSeconds :type Float%20%28double-precision%29) (TriggeredSeconds :type Float%20%28double-precision%29) (InputAction :type Input%20Action%20Object%20Reference :default "/Game/Game/Inputs/Weapons/IA_SecondaryLeft.IA_SecondaryLeft"))
  (if (GameplayTags|HasTag (Variables|Default|GetCharacterTags) "(TagName=\"CharacterStatus.CanMove\")")
    (CallFunction|FireSecondaryLeft)))

(event Input|EnhancedActionEvents|EnhancedInputActionIA_SecondaryRight
  (params (ActionValue :type Boolean) (ElapsedSeconds :type Float%20%28double-precision%29) (TriggeredSeconds :type Float%20%28double-precision%29) (InputAction :type Input%20Action%20Object%20Reference :default "/Game/Game/Inputs/Weapons/IA_SecondaryRight.IA_SecondaryRight"))
  (if (GameplayTags|HasTag (Variables|Default|GetCharacterTags) "(TagName=\"CharacterStatus.CanMove\")")
    (CallFunction|FireSecondaryRight)))

(event Input|EnhancedActionEvents|EnhancedInputActionIA_Look
  (params (ActionValue :type Vector%202D%20Structure) (ElapsedSeconds :type Float%20%28double-precision%29) (TriggeredSeconds :type Float%20%28double-precision%29) (InputAction :type Input%20Action%20Object%20Reference :default "/Game/Game/Inputs/IA_Look.IA_Look"))
  (if (GameplayTags|HasTag (Variables|Default|GetCharacterTags) "(TagName=\"CharacterStatus.CanMove\")")
    (Pawn|Input|AddControllerYawInput (.x ActionValue))
    (Pawn|Input|AddControllerPitchInput (.y ActionValue))))

(event Input|EnhancedActionEvents|EnhancedInputActionIA_Movement
  (params (ActionValue :type Vector%202D%20Structure) (ElapsedSeconds :type Float%20%28double-precision%29) (TriggeredSeconds :type Float%20%28double-precision%29) (InputAction :type Input%20Action%20Object%20Reference :default "/Game/Game/Inputs/IA_Movement.IA_Movement"))
  (if (GameplayTags|HasTag (Variables|Default|GetCharacterTags) "(TagName=\"CharacterStatus.CanMove\")")
    (Pawn|Input|AddMovementInput (Transformation|GetActorRightVector) (.x ActionValue) false)
    (Pawn|Input|AddMovementInput (Transformation|GetActorForwardVector) (.y ActionValue) false)
    (Variables|Default|SetMovementAxis (Math|Vector2D|MakeVector2D (.x ActionValue) (.y ActionValue)))))

(event Input|EnhancedActionEvents|EnhancedInputActionIA_Crouch
  (params (ActionValue :type Boolean) (ElapsedSeconds :type Float%20%28double-precision%29) (TriggeredSeconds :type Float%20%28double-precision%29) (InputAction :type Input%20Action%20Object%20Reference :default "/Game/Game/Inputs/IA_Crouch.IA_Crouch"))
  (:Triggered
    (if (GameplayTags|HasTag (Variables|Default|GetCharacterTags) "(TagName=\"CharacterStatus.CanMove\")")
      (CallFunction|CharacterCrouch)))
  (:Canceled
    (CallFunction|CharacterStopCrouch :!label _label))
  (:Completed
    (goto _label)))

(event Input|EnhancedActionEvents|EnhancedInputActionIA_Jump
  (params (ActionValue :type Boolean) (ElapsedSeconds :type Float%20%28double-precision%29) (TriggeredSeconds :type Float%20%28double-precision%29) (InputAction :type Input%20Action%20Object%20Reference :default "/Game/Game/Inputs/IA_Jump.IA_Jump"))
  (bind _charactertags (Variables|Default|GetCharacterTags))
  (bind _currentjumps (Variables|Default|GetCurrentJumps))
  (bind _charactertags_2 (Variables|Default|GetCharacterTags))
  (bind _charactermovement (Variables|Character|GetCharacterMovement))
  (bind _velocity (Variables|/Script/Engine.MovementComponent|GetVelocity _charactermovement))
  (:Triggered
    (if (and (GameplayTags|HasTag _charactertags "(TagName=\"CharacterStatus.CanMove\")") (not (GameplayTags|HasTag _charactertags "(TagName=\"CharacterStatus.Jumping\")")))
      (if (> _currentjumps 0)
        (GameplayTags|AddGameplayTag _charactertags_2 "(TagName=\"CharacterStatus.Jumping\")" :!class /Script/GameplayTags.BlueprintGameplayTagLibrary)
        (Character|UnCrouch)
        (Utilities|FlowControl|Delay 0.001)
        (switch int _currentjumps
          (:1
            (Audio|PlaySound2D "/Game/GameAssets/Audio/boost.boost" 0.25 1.0 0.0 0 0)
            (Character|LaunchCharacter (Math|Vector|MakeVector (* (.x _velocity) 0.5) (* (.y _velocity) 0.5) 2e+03) true true))
          (:2
            (Audio|PlaySound2D "/Game/GameAssets/Audio/footstep_02.footstep_02" 0.5 0.85 0.0 0 0)
            (Character|Jump)))
        (Math|Integer|DecrementInt _currentjumps))))
  (:Canceled
    (Character|StopJumping :!label _label)
    (GameplayTags|RemoveGameplayTag _charactertags_2 "(TagName=\"CharacterStatus.Jumping\")" :!class /Script/GameplayTags.BlueprintGameplayTagLibrary)
    (Variables|/Script/Engine.CharacterMovementComponent|SetGravityScale (Variables|Character|GetCharacterMovement) 4.0))
  (:Completed
    (goto _label)))

(event Input|KeyboardEvents|DebugKeyP
  (params (Key :type Key%20Structure :default "None") (ActionValue :type Input%20Action%20Value%20Structure))
  (bind _charactertags (Variables|Default|GetCharacterTags))
  (:Pressed
    (Utilities|FlowControl|FlipFlop
      (:A
        (GameplayTags|AddGameplayTag _charactertags "(TagName=\"CharacterStatus.Damageable\")" :!class /Script/GameplayTags.BlueprintGameplayTagLibrary)
        (Development|PrintString "INVINCIBILITY DEACTIVATED"))
      (:B
        (GameplayTags|RemoveGameplayTag _charactertags "(TagName=\"CharacterStatus.Damageable\")" :!class /Script/GameplayTags.BlueprintGameplayTagLibrary)
        (Development|PrintString "INVINCIBILITY ACTIVATED")))))

(event Input|KeyboardEvents|L
  (params (Key :type Key%20Structure :default "None"))
  (:Pressed
    (CallFunction|AttachWeapon "/Game/Game/Blueprints/Weapons/ShoulderCannon/BP_ShoulderCannon.BP_ShoulderCannon_C" "NewEnumerator1" true)))

(event Input|KeyboardEvents|K
  (params (Key :type Key%20Structure :default "None"))
  (:Pressed
    (CallFunction|AttachWeapon "/Game/Game/Blueprints/Weapons/MachineGun/BP_MachineGun.BP_MachineGun_C" "NewEnumerator0" true)))