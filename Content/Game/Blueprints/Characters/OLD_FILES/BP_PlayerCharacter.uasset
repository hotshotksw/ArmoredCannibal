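; Player character from the OLD_FILES folder with Enhanced Input movement, four weapon slots and a HUD created on BeginPlay.
; AttachWeapon fills free primary or secondary arrow mounts with weapon components, each fired by its own input.
; Jumping chains into a launch boost; crouching shrinks the capsule by timeline and drops ground friction for sliding.
; Debug keys attach test weapons, and P animates a cel-shader filter through a material parameter collection.
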(event `Key|P` :paused true
  (params (Key :type "Key Structure"))
  (:`Pressed`
    (bind (_direction _filterlevel) (`Timeline|Lerp Filter` :!via `PlayFromStart`)
      (:`Update`
        (`KismetMaterialLibrary.SetScalarParameterValue` "/Game/Game/Materials/Shaders/CelShader/CelShaderParameters.CelShaderParameters" "AlphaFilterStrength" (`KismetMathLibrary.Lerp` 0.0 1.0 _filterlevel))
        (`KismetSystemLibrary.Delay` 5.0)
        (bind (_direction_2 _filterlevel_2) (`Timeline|Timeline` :!via `PlayFromStart`)
          (:`Update`
            (`KismetMaterialLibrary.SetScalarParameterValue` "/Game/Game/Materials/Shaders/CelShader/CelShaderParameters.CelShaderParameters" "AlphaFilterStrength" (`KismetMathLibrary.Lerp` 1.0 0.0 _filterlevel_2))))))))

(event `self.ReceiveBeginPlay`
  (bind _returnvalue (`|CreateWidget` "/Game/Game/Blueprints/Visual/PlayerHUD/W_PlayerHUD.W_PlayerHUD_C"))
  (`UserWidget.AddToViewport` _returnvalue 0))

(event `self.ReceiveTick`
  (params (DeltaSeconds :type "Float (single-precision)")))

(event `EnhancedInput|/Game/Game/Inputs/IA_Look`
  (params (ActionValue :type "Vector2D Structure") (ElapsedSeconds :type "Float (double-precision)") (TriggeredSeconds :type "Float (double-precision)") (InputAction :type "InputAction Object Reference" :default "/Game/Game/Inputs/IA_Look.IA_Look"))
  (:`Triggered`
    (`self.AddControllerYawInput` ActionValue_X)
    (`self.AddControllerPitchInput` ActionValue_Y)))

(event `EnhancedInput|/Game/Game/Inputs/IA_Jump`
  (params (ActionValue :type Boolean) (ElapsedSeconds :type "Float (double-precision)") (TriggeredSeconds :type "Float (double-precision)") (InputAction :type "InputAction Object Reference" :default "/Game/Game/Inputs/IA_Jump.IA_Jump"))
  (bind _currentjumps (`self.CurrentJumps`))
  (bind (_velocity_x _velocity_y) (`KismetMathLibrary.BreakVector` (`MovementComponent.Velocity` (`self.CharacterMovement`))))
  (:`Started`
    (if (> _currentjumps 0)
      (`self.UnCrouch`)
      (`KismetSystemLibrary.Delay` 0.001)
      (if (== _currentjumps 2)
        (`GameplayStatics.PlaySound2D` null 1.0 1.0 0.0 null null)
        (`self.Jump`)
        (else
          (`GameplayStatics.PlaySound2D` "/Game/Game/Audio/boost.boost" 0.5 1.0 0.0 null null)
          (`self.LaunchCharacter` (`KismetMathLibrary.MakeVector` (* _velocity_x 0.5) (* _velocity_y 0.5) 2000.0) true true)))
      (`/Engine/EditorBlueprintResources/StandardMacros.DecrementInt` _currentjumps
        (:`  `
          (`KismetSystemLibrary.PrintString` (`KismetStringLibrary.Concat_StrStr` "Jumps Remaining: " (`KismetStringLibrary.Conv_IntToString` _currentjumps)))))))
  (:`Canceled`
    (`self.StopJumping` :!label _label)
    (set `CharacterMovementComponent.GravityScale` 4.0 (`self.CharacterMovement`)))
  (:`Completed`
    (goto _label)))

(event `Key|L`
  (params (Key :type "Key Structure"))
  (:`Pressed`
    (`self.AttachWeapon` "/Game/Game/Blueprints/Weapons/ShoulderCannon/BP_ShoulderCannon.BP_ShoulderCannon_C" "NewEnumerator1")))

(event `Key|K`
  (params (Key :type "Key Structure"))
  (:`Pressed`
    (`self.AttachWeapon` "/Game/Game/Blueprints/Weapons/MachineGun/BP_MachineGun.BP_MachineGun_C")))

(event `EnhancedInput|/Game/Game/Inputs/IA_Movement`
  (params (ActionValue :type "Vector2D Structure") (ElapsedSeconds :type "Float (double-precision)") (TriggeredSeconds :type "Float (double-precision)") (InputAction :type "InputAction Object Reference" :default "/Game/Game/Inputs/IA_Movement.IA_Movement"))
  (:`Triggered`
    (`self.AddMovementInput` (`self.GetActorRightVector`) ActionValue_X)
    (`self.AddMovementInput` (`self.GetActorForwardVector`) ActionValue_Y)
    (set `self.MovementAxis` (`KismetMathLibrary.MakeVector2D` ActionValue_X ActionValue_Y))))

(event `EnhancedInput|/Game/Game/Inputs/Weapons/IA_PrimaryRight`
  (params (ActionValue :type Boolean) (ElapsedSeconds :type "Float (double-precision)") (TriggeredSeconds :type "Float (double-precision)") (InputAction :type "InputAction Object Reference" :default "/Game/Game/Inputs/Weapons/IA_PrimaryRight.IA_PrimaryRight"))
  (bind _primaryright (`self.PrimaryRight`))
  (:`Triggered`
    (`/Engine/EditorBlueprintResources/StandardMacros.IsValid` _primaryright
      (:`Is Valid`
        (`/Game/Game/Blueprints/ActorComponents/WeaponComponent.FireWeapon` _primaryright)))))

(event `EnhancedInput|/Game/Game/Inputs/Weapons/IA_PrimaryLeft`
  (params (ActionValue :type Boolean) (ElapsedSeconds :type "Float (double-precision)") (TriggeredSeconds :type "Float (double-precision)") (InputAction :type "InputAction Object Reference" :default "/Game/Game/Inputs/Weapons/IA_PrimaryLeft.IA_PrimaryLeft"))
  (bind _primaryleft (`self.PrimaryLeft`))
  (:`Triggered`
    (`/Engine/EditorBlueprintResources/StandardMacros.IsValid` _primaryleft
      (:`Is Valid`
        (`/Game/Game/Blueprints/ActorComponents/WeaponComponent.FireWeapon` _primaryleft)))))

(event `EnhancedInput|/Game/Game/Inputs/Weapons/IA_SecondaryLeft`
  (params (ActionValue :type Boolean) (ElapsedSeconds :type "Float (double-precision)") (TriggeredSeconds :type "Float (double-precision)") (InputAction :type "InputAction Object Reference" :default "/Game/Game/Inputs/Weapons/IA_SecondaryLeft.IA_SecondaryLeft"))
  (bind _secondaryleft (`self.SecondaryLeft`))
  (:`Triggered`
    (`/Engine/EditorBlueprintResources/StandardMacros.IsValid` _secondaryleft
      (:`Is Valid`
        (`/Game/Game/Blueprints/ActorComponents/WeaponComponent.FireWeapon` _secondaryleft)))))

(event `EnhancedInput|/Game/Game/Inputs/Weapons/IA_SecondaryRight`
  (params (ActionValue :type Boolean) (ElapsedSeconds :type "Float (double-precision)") (TriggeredSeconds :type "Float (double-precision)") (InputAction :type "InputAction Object Reference" :default "/Game/Game/Inputs/Weapons/IA_SecondaryRight.IA_SecondaryRight"))
  (bind _secondaryright (`self.SecondaryRight`))
  (:`Triggered`
    (`/Engine/EditorBlueprintResources/StandardMacros.IsValid` _secondaryright
      (:`Is Valid`
        (`/Game/Game/Blueprints/ActorComponents/WeaponComponent.FireWeapon` _secondaryright)))))

(event `self.OnLanded`
  (params (Hit :type "HitResult Structure (by ref)"))
  (bind _output_get (set `self.CurrentJumps` (`CharacterMovementComponent.MaxJumpApexAttemptsPerSimulation` (`self.CharacterMovement`))))
  (`KismetSystemLibrary.PrintString` (`KismetStringLibrary.Concat_StrStr` "Jumps Remaining: " (`KismetStringLibrary.Conv_IntToString` _output_get))))

(event `EnhancedInput|/Game/Game/Inputs/IA_Crouch`
  (params (ActionValue :type Boolean) (ElapsedSeconds :type "Float (double-precision)") (TriggeredSeconds :type "Float (double-precision)") (InputAction :type "InputAction Object Reference" :default "/Game/Game/Inputs/IA_Crouch.IA_Crouch"))
  (bind _charactermovement (`self.CharacterMovement`))
  (:`Triggered`
    (set `self.IsCrouched` true)
    (if (!= (`CharacterMovementComponent.GroundFriction` _charactermovement) 0.4)
      (set `CharacterMovementComponent.GroundFriction` 0.0 _charactermovement)
      (set `CharacterMovementComponent.GravityScale` 4.0 _charactermovement)
      (bind (_direction _crouch) (`Timeline|Timeline_Crouch` :!label _label_2)
        (:`Update`
          (`CapsuleComponent.SetCapsuleHalfHeight` (`self.CapsuleComponent`) (`KismetMathLibrary.Lerp` 130.0 25.0 _crouch) true)))))
  (:`Canceled`
    (set `self.IsCrouched` false :!label _label_3)
    (set `CharacterMovementComponent.GroundFriction` 8.0 _charactermovement)
    (set `CharacterMovementComponent.GravityScale` 2.0 _charactermovement)
    (goto _label_2 :!via `Reverse`))
  (:`Completed`
    (goto _label_3)))

(fn `AttachWeapon`
  (params (NewWeapon :type "/Game/Game/Blueprints/Weapons/Master/BP_WeaponBase Class Reference") (WeaponPosition :type "/Game/Game/Blueprints/Weapons/Master/E_WeaponPosition Enum" :default "NewEnumerator0"))
  (if (`|EnumEquality` WeaponPosition "NewEnumerator0")
    ;[0.1927 0 0] Primary Weapon Addition
    (`/Engine/EditorBlueprintResources/StandardMacros.IsValid` (`self.PrimaryRight`)
      (:`Is Valid`
        (`/Engine/EditorBlueprintResources/StandardMacros.IsValid` (`self.PrimaryLeft`)
          (:`Is Not Valid`
            (bind _returnvalue (`AddComponent|NODE_AddWeaponComponent-0`))
            (bind _output_get (set `self.PrimaryLeft` _returnvalue))
            (`/Game/Game/Blueprints/ActorComponents/WeaponComponent.AttachWeapon` _output_get NewWeapon (`self.PrimaryLeftArrow`)))))
      (:`Is Not Valid`
        (bind _returnvalue_2 (`AddComponent|NODE_AddWeaponComponent-1`))
        (bind _output_get_2 (set `self.PrimaryRight` _returnvalue_2))
        (`/Game/Game/Blueprints/ActorComponents/WeaponComponent.AttachWeapon` _output_get_2 NewWeapon (`self.PrimaryRightArrow`))))
    (else
      ;[0.03049 0.01628 0.1562] Secondary Weapon Addition
      (`/Engine/EditorBlueprintResources/StandardMacros.IsValid` (`self.SecondaryLeft`)
        (:`Is Valid`
          (`/Engine/EditorBlueprintResources/StandardMacros.IsValid` (`self.SecondaryRight`)
            (:`Is Not Valid`
              (bind _returnvalue_3 (`AddComponent|NODE_AddWeaponComponent-2`))
              (bind _output_get_3 (set `self.SecondaryRight` _returnvalue_3))
              (`/Game/Game/Blueprints/ActorComponents/WeaponComponent.AttachWeapon` _output_get_3 NewWeapon (`self.SecondaryRightArrow`)))))
        (:`Is Not Valid`
          (bind _returnvalue_4 (`AddComponent|NODE_AddWeaponComponent-3`))
          (bind _output_get_4 (set `self.SecondaryLeft` _returnvalue_4))
          (`/Game/Game/Blueprints/ActorComponents/WeaponComponent.AttachWeapon` _output_get_4 NewWeapon (`self.SecondaryLeftArrow`)))))))

(fn `CanJumpInternal`
  (returns (ReturnValue :type Boolean))
  (return true))

(fn `UserConstructionScript`)