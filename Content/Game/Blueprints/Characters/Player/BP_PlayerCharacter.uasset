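; BP_PlayerCharacter is the player character Blueprint, handling look, movement, jump and a directional boost through Enhanced Input.
; Boost launches the character along the current movement input relative to its facing, overriding horizontal velocity and keeping vertical velocity.
; AddToBoostMeter increments a clamped boost meter, but boosting neither checks nor spends it, as that logic is disconnected.
; Debug keys fill and print the meter.
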(event Custom|AddToBoostMeter
  (bind _result (Math|Integer|IncrementInt (Variables|Default|GetBoostMeter))
    (:%20%20
      (Variables|Default|SetBoostMeter (Math|Integer|Clamp(Integer) _result 0 100)))))

(event Input|EnhancedActionEvents|EnhancedInputActionIA_Look
  (params (ActionValue :type Vector%202D%20Structure) (ElapsedSeconds :type Float%20%28double-precision%29) (TriggeredSeconds :type Float%20%28double-precision%29) (InputAction :type Input%20Action%20Object%20Reference :default "/Game/Game/Inputs/IA_Look.IA_Look"))
  (Pawn|Input|AddControllerYawInput (.x ActionValue))
  (Pawn|Input|AddControllerPitchInput (.y ActionValue)))

(event Input|EnhancedActionEvents|EnhancedInputActionIA_Movement
  (params (ActionValue :type Vector%202D%20Structure) (ElapsedSeconds :type Float%20%28double-precision%29) (TriggeredSeconds :type Float%20%28double-precision%29) (InputAction :type Input%20Action%20Object%20Reference :default "/Game/Game/Inputs/IA_Movement.IA_Movement"))
  (Pawn|Input|AddMovementInput (Transformation|GetActorRightVector) (.x ActionValue) false)
  (Pawn|Input|AddMovementInput (Transformation|GetActorForwardVector) (.y ActionValue) false))

(event Input|EnhancedActionEvents|EnhancedInputActionIA_Jump
  (params (ActionValue :type Boolean) (ElapsedSeconds :type Float%20%28double-precision%29) (TriggeredSeconds :type Float%20%28double-precision%29) (InputAction :type Input%20Action%20Object%20Reference :default "/Game/Game/Inputs/IA_Jump.IA_Jump"))
  (:Started
    (Character|Jump))
  (:Completed
    (Character|StopJumping)))

(event Input|EnhancedActionEvents|EnhancedInputActionIA_Boost
  (params (ActionValue :type Boolean) (ElapsedSeconds :type Float%20%28double-precision%29) (TriggeredSeconds :type Float%20%28double-precision%29) (InputAction :type Input%20Action%20Object%20Reference :default "/Game/Game/Inputs/IA_Boost.IA_Boost"))
  (bind _returnvalue (Input|EnhancedActionValues|GetIA_Movement))
  (Character|LaunchCharacter (* (+ (* (Transformation|GetActorRightVector) (.x _returnvalue)) (* (.y _returnvalue) (Transformation|GetActorForwardVector))) 2e+03) true false))

(event EventBeginPlay)

(event Collision|EventActorBeginOverlap
  (params (OtherActor :type Actor%20Object%20Reference)))

(event EventTick
  (params (DeltaSeconds :type Float%20%28single-precision%29)))

(event Input|KeyboardEvents|DebugKeyB
  (params (Key :type Key%20Structure :default "None") (ActionValue :type Input%20Action%20Value%20Structure))
  (:Pressed
    (Development|PrintText (Utilities|Text|ToText(Integer) (Variables|Default|GetBoostMeter)))))

(event Input|KeyboardEvents|DebugKeyM
  (params (Key :type Key%20Structure :default "None") (ActionValue :type Input%20Action%20Value%20Structure))
  (:Pressed
    (Variables|Default|SetBoostMeter 100)))

(fn ConstructionScript)