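; Actor component that gives the player character a charge-limited directional boost on the ground or in the air, shown on a gauge widget.
; On BeginPlay it adds the boost input mapping and creates the gauge.
; Boost input launches the character along weighted movement input, spends charge and briefly drops gravity in air or friction on ground, with DoOnce blocking overlaps.
; Debug keys refill charge and toggle infinite boost.
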(event EventBeginPlay
  (bind _asbp_character_base (Utilities|Casting|CastToBP_CharacterBase (Components|GetOwner)))
  (bind _output_get (Variables|Default|SetCharacter _asbp_character_base))
  (bind _asbp_player_controller (Utilities|Casting|CastToBP_PlayerController (Pawn|GetController _output_get)))
  (Utilities|IsValid (PlayerController|LocalPlayerSubsystems|GetEnhancedInputLocalPlayerSubsystem _asbp_player_controller)
    (:Is%20Valid
      (Input|AddMappingContext (PlayerController|LocalPlayerSubsystems|GetEnhancedInputLocalPlayerSubsystem _asbp_player_controller) "/Game/Game/Inputs/Boost/IMC_Boost.IMC_Boost" 0 "(bIgnoreAllPressedKeysUntilRelease=True,bForceImmediately=False,bNotifyUserSettings=False)")
      (bind _returnvalue (UserInterface|CreateWidget "/Game/Game/Blueprints/Visual/PlayerHUD/W_BoostGauge.W_BoostGauge_C"))
      (bind _output_get_2 (Variables|Default|SetBoostWidget _returnvalue))
      (CallFunction|ChangeBoostValue (Variables|Default|GetMaxBoost))
      (UserInterface|Viewport|AddtoViewport _output_get_2 0))))

(event EventTick
  (params (DeltaSeconds :type Float%20%28single-precision%29)))

(fn ActivateBoost
  (bind _airboostvalue (Variables|Default|GetAirBoostValue))
  (bind _groundboostvalue (Variables|Default|GetGroundBoostValue))
  (bind _character (Variables|Default|GetCharacter))
  (bind _returnvalue (Transformation|GetActorRightVector _character))
  (bind _returnvalue_2 (Transformation|GetActorForwardVector _character))
  (bind _movementaxis (Variables|/Game/Game/Blueprints/Characters/Master/BP_CharacterBase.BP_CharacterBase_C|GetMovementAxis _character))
  (bind _charactermovement (Variables|/Script/Engine.Character|GetCharacterMovement _character))
  (bind _returnvalue_3 (AI|Components|NavMovement|IsFalling _charactermovement))
  (bind _returnvalue_4 (* (.x _movementaxis) 2.0))
  (bind _returnvalue_5 (* (.y _movementaxis) _returnvalue_2))
  (bind _returnvalue_6 (* _returnvalue _returnvalue_4))
  (bind _returnvalue_7 (+ _returnvalue_6 _returnvalue_5))
  (bind _returnvalue_8 (Math|Vector|Normalize _returnvalue_7))
  (bind _returnvalue_9 (* _returnvalue_8 _groundboostvalue))
  (bind _returnvalue_10 (* _airboostvalue _returnvalue_8))
  (if _returnvalue_3
    (Character|LaunchCharacter _character (Math|Vector|MakeVector (.x _returnvalue_10) (.y _returnvalue_10) 1e+02) true true)
    (else
      (Character|LaunchCharacter _character (Math|Vector|MakeVector (.x _returnvalue_9) (.y _returnvalue_9) 0.0) true false)))
  (if (Variables|Default|GetInfiniteBoost)
    _
    (else
      (CallFunction|ChangeBoostValue -50)))
  (Default|CallOnBoost)
  (Audio|PlaySound2D "/Game/Game/Audio/boost.boost" 0.35 2.0 0.0 0 0)
  (return _returnvalue_3))

(fn RemoveBoost
  (Widget|RemovefromParent (Variables|Default|GetBoostWidget))
  (Components|DestroyComponent))

(event Custom|ChangeBoostValue
  (params (Value :type Integer))
  (bind _output_get (Variables|Default|SetBoostPercentage (Math|Integer|Clamp(Integer) (+ (Variables|Default|GetBoostPercentage) Value) 0 (Variables|Default|GetMaxBoost))))
  (Default|ChangeSliderValue (Variables|Default|GetBoostWidget) (/ _output_get (Variables|Default|GetMaxBoost)))
  (Development|PrintString (Utilities|String|Append "Current Boost Charges: " (Utilities|String|ToString(Integer) _output_get))))

(event Input|EnhancedActionEvents|EnhancedInputActionIA_Boost
  (params (ActionValue :type Boolean) (ElapsedSeconds :type Float%20%28double-precision%29) (TriggeredSeconds :type Float%20%28double-precision%29) (InputAction :type Input%20Action%20Object%20Reference :default "/Game/Game/Inputs/Boost/IA_Boost.IA_Boost"))
  (bind _character (Variables|Default|GetCharacter))
  (bind _charactermovement (Variables|/Script/Engine.Character|GetCharacterMovement _character))
  (if (and (> (Variables|Default|GetBoostPercentage) 0) (Utilities|Operators|NotEqual(!=) :A (Variables|/Script/Engine.MovementComponent|GetVelocity _charactermovement)))
    (Utilities|FlowControl|DoOnce false :!label _label
      (:Completed
        (bind _airborne (CallFunction|ActivateBoost))
        (if _airborne
          (Variables|/Script/Engine.CharacterMovementComponent|SetGravityScale _charactermovement 0.0)
          (Utilities|FlowControl|Delay 0.25)
          (Variables|/Script/Engine.CharacterMovementComponent|SetGravityScale _charactermovement 4.0)
          (goto _label Reset)
          (else
            (Variables|/Script/Engine.CharacterMovementComponent|SetGroundFriction _charactermovement 0.4)
            (Utilities|FlowControl|Delay 0.2)
            (Variables|/Script/Engine.CharacterMovementComponent|SetGroundFriction _charactermovement 8.0)
            (goto _label Reset)))))))

(event Input|KeyboardEvents|DebugKeyB
  (params (Key :type Key%20Structure :default "None") (ActionValue :type Input%20Action%20Value%20Structure))
  (:Pressed
    (bind _output_get (Variables|Default|SetInfiniteBoost (not (Variables|Default|GetInfiniteBoost))))
    (Development|PrintString (Utilities|String|Append "Infinite Boost: " (Utilities|String|ToString(Boolean) _output_get)))))

(event Input|KeyboardEvents|DebugKeyM
  (params (Key :type Key%20Structure :default "None") (ActionValue :type Input%20Action%20Value%20Structure))
  (:Pressed
    (CallFunction|ChangeBoostValue 9999)))