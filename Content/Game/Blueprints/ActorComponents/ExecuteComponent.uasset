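; Enemy actor component that runs a player-triggered execution finisher on its owning BP_Enemy.
; AttachExecuteSphere spawns a BP_ExecuteCollision on the owner's capsule and binds its executing event; Start requires an overlapped player and fires once.
; Start snaps the player's mesh to the enemy's ExecuteDirection, swaps gameplay tags to block movement and damage, and plays the player's ActorSequence.
; After fixed delays it restores the player, destroys sphere and component, and kills the enemy.
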(event `self.ReceiveBeginPlay`
  (bind _asbp_enemy (cast `/Game/Game/Blueprints/Characters/Enemy/BP_Enemy` (`self.GetOwner`)))
  (set `self.Executee` _asbp_enemy))

(event `self.ReceiveTick`
  (params (DeltaSeconds :type "Float (single-precision)")))

(event `AttachExecuteSphere`
  (params (Owner :type "/Game/Game/Blueprints/Characters/Master/BP_CharacterBase Object Reference"))
  (bind _capsulecomponent (`Character.CapsuleComponent` Owner))
  (bind _returnvalue (`|SpawnActorFromClass` "/Game/Game/Blueprints/Objects/BP_ExecuteCollision.BP_ExecuteCollision_C" (`SceneComponent.K2_GetComponentToWorld` _capsulecomponent) "Undefined" "MultiplyWithRoot" null null))
  (bind _output_get (set `self.ExecuteSphere` _returnvalue))
  (add `/Game/Game/Blueprints/Objects/BP_ExecuteCollision.OnExecutingSphere` _output_get (`|CreateDelegate` :!event `Start`))
  (`SceneComponent.K2_AttachToComponent` (`Actor.RootComponent` _output_get) _capsulecomponent "None" "SnapToTarget" "KeepRelative" "KeepRelative" true))

(event `Start`
  (bind _executer (`self.Executer`))
  (bind _executer_2 (`self.Executer`))
  (bind _executer_3 (`self.Executer`))
  (bind _executer_4 (`self.Executer`))
  (bind _charactertags (`/Game/Game/Blueprints/Characters/Master/BP_CharacterBase.CharacterTags` _executer_3))
  (bind _charactertags_2 (`/Game/Game/Blueprints/Characters/Master/BP_CharacterBase.CharacterTags` (`self.Executer`)))
  (bind _mesh (`Character.Mesh` _executer_2))
  (bind _executesphere (`self.ExecuteSphere`)
    (:`then`
      (bind _overlappedplayer (`/Game/Game/Blueprints/Objects/BP_ExecuteCollision.OverlappedPlayer` _executesphere)
        (:`then`
          (`/Engine/EditorBlueprintResources/StandardMacros.DoOnce` false
            (:`Completed`
              (set `self.Executer` _overlappedplayer)
              (`Widget.RemoveFromParent` (`/Game/Game/Blueprints/Objects/BP_ExecuteCollision.ExecuteWidget` (`self.ExecuteSphere`)))
              (`GameplayStatics.PlaySound2D` "/Game/Game/Audio/execute_activation.execute_activation" 1.0 1.0 0.0 null null)
              (`KismetSystemLibrary.Delay` 0.5)
              (`BlueprintGameplayTagLibrary.AddGameplayTag` (`/Game/Game/Blueprints/Characters/Master/BP_CharacterBase.CharacterTags` (`self.Executee`)) (struct :`TagName` "CharacterStatus.Executed"))
              (set `MovementComponent.Velocity` (0.0 0.0 0.0) (`Character.CharacterMovement` _executer_4))
              (`SceneComponent.K2_SetWorldTransform` (`Character.Mesh` _executer_4) (`SceneComponent.K2_GetComponentToWorld` (`/Game/Game/Blueprints/Characters/Enemy/BP_Enemy.ExecuteDirection` (`self.Executee`))) false false)
              (`BlueprintGameplayTagLibrary.RemoveGameplayTag` _charactertags_2 (struct :`TagName` "CharacterStatus.CanMove"))
              (`BlueprintGameplayTagLibrary.AddGameplayTag` _charactertags_2 (struct :`TagName` "CharacterStatus.Executed"))
              (`BlueprintGameplayTagLibrary.RemoveGameplayTag` _charactertags_2 (struct :`TagName` "CharacterStatus.Damageable"))
              (`ActorSequenceComponent.PlaySequence` (`/Game/Game/Blueprints/Characters/Master/BP_Player.ActorSequence` _executer))
              (set `CameraComponent.bUsePawnControlRotation` false (`/Game/Game/Blueprints/Characters/Master/BP_CharacterBase.Camera` _executer))
              (`KismetSystemLibrary.Delay` 3.05)
              (`ActorSequenceComponent.StopSequence` (`/Game/Game/Blueprints/Characters/Master/BP_Player.ActorSequence` _executer_3))
              (`BlueprintGameplayTagLibrary.RemoveGameplayTag` _charactertags (struct :`TagName` "CharacterStatus.Executed"))
              (`BlueprintGameplayTagLibrary.AddGameplayTag` _charactertags (struct :`TagName` "CharacterStatus.CanMove"))
              (`BlueprintGameplayTagLibrary.AddGameplayTag` _charactertags (struct :`TagName` "CharacterStatus.Damageable"))
              (`SceneComponent.ResetRelativeTransform` _mesh)
              (`SceneComponent.K2_SetRelativeLocation` _mesh (`/Game/Game/Blueprints/Characters/Master/BP_Player.MeshPosition` _executer_2) false false)
              (set `CameraComponent.bUsePawnControlRotation` true (`/Game/Game/Blueprints/Characters/Master/BP_CharacterBase.Camera` (`self.Executer`)))
              (`self.DestroyExecute`)
              (`/Game/Game/Blueprints/Characters/Enemy/BP_Enemy.KillEnemy` (`self.Executee`)))))
        (:`else`)))
    (:`else`)))

(event `DestroyExecute`
  (bind _executesphere (`self.ExecuteSphere`)
    (:`then`
      (`Actor.K2_DestroyActor` _executesphere))
    (:`else`
      _))
  (`self.K2_DestroyComponent`))

(fn `StartExecute`
  (returns (Executed :type Boolean)))