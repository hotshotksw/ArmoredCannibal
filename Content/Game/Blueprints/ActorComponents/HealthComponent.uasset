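; Actor component that tracks health for BP_CharacterBase owners, handling damage, healing, death notification and health bar creation.
; TakeDamage applies only while the owner has the CharacterStatus.Damageable gameplay tag, then fires damage and death dispatchers; debug key P toggles that tag.
; The player gets a viewport widget updated on damage and healing.
; Enemies get a runtime screen-space WidgetComponent seeded with their current health values.
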(event Custom|CreatePlayerHealthbar
  (bind _returnvalue (UserInterface|CreateWidget "/Game/Game/Blueprints/Visual/PlayerHUD/W_PlayerHealth.W_PlayerHealth_C"))
  (bind _output_get (Variables|Default|SetPlayerHealthBar _returnvalue))
  (bind _output_get_2 (Variables|/Game/Game/Blueprints/Visual/PlayerHUD/W_PlayerHealth.W_PlayerHealth_C|SetMaxHealth _output_get (Variables|Default|GetMaxHealth)))
  (Default|ChangeSliderValue (Variables|Default|GetPlayerHealthBar) _output_get_2)
  (UserInterface|Viewport|AddtoViewport (Variables|Default|GetPlayerHealthBar) 0))

(event Custom|CreateEnemyHealthbar
  (bind _returnvalue (Game|AddComponentbyClass (Components|GetOwner) "/Script/UMG.WidgetComponent" false (Math|Transform|MakeTransform "0.000000,0.000000,135.000000" "0, 0, 0" "1.000000,1.000000,1.000000")))
  (Class|WidgetComponent|SetDrawSize _returnvalue "(X=1.000000,Y=1.000000)")
  (Class|WidgetComponent|SetWidgetSpace _returnvalue "Screen")
  (Collision|SetCollisionEnabled _returnvalue "NoCollision")
  (bind _returnvalue_2 (UserInterface|CreateWidget "/Game/Game/Blueprints/Visual/Enemy/W_EnemyHealth.W_EnemyHealth_C"))
  (Variables|Default|SetEnemyHealthBar _returnvalue_2)
  (bind _asbp_enemy (Utilities|Casting|CastToBP_Enemy (Components|GetOwner)))
  (Variables|/Game/Game/Blueprints/Visual/Enemy/W_EnemyHealth.W_EnemyHealth_C|SetCharacter (Variables|Default|GetEnemyHealthBar) _asbp_enemy)
  (Variables|/Game/Game/Blueprints/Visual/Enemy/W_EnemyHealth.W_EnemyHealth_C|SetHealth (Variables|Default|GetEnemyHealthBar) (Variables|Default|GetHealth))
  (Variables|/Game/Game/Blueprints/Visual/Enemy/W_EnemyHealth.W_EnemyHealth_C|SetMaxHealth (Variables|Default|GetEnemyHealthBar) (Variables|Default|GetMaxHealth))
  (UserInterface|SetWidget _returnvalue (Variables|Default|GetEnemyHealthBar)))

(event EventBeginPlay
  (Variables|Default|SetHealth (Variables|Default|GetMaxHealth))
  (bind _asbp_character_base (Utilities|Casting|CastToBP_CharacterBase (Components|GetOwner)))
  (Variables|Default|SetOwner _asbp_character_base))

(event Input|KeyboardEvents|DebugKeyP
  (params (Key :type Key%20Structure) (ActionValue :type Input%20Action%20Value%20Structure))
  (bind _owner (Variables|Default|GetOwner))
  (bind _charactertags (Variables|/Game/Game/Blueprints/Characters/Master/BP_CharacterBase.BP_CharacterBase_C|GetCharacterTags _owner))
  (:Pressed
    (if (GameplayTags|HasTag (Variables|/Game/Game/Blueprints/Characters/Master/BP_CharacterBase.BP_CharacterBase_C|GetCharacterTags (Variables|Default|GetOwner)) "(TagName=\"CharacterStatus.Damageable\")")
      (GameplayTags|RemoveGameplayTag _charactertags "(TagName=\"CharacterStatus.Damageable\")" :!class /Script/GameplayTags.BlueprintGameplayTagLibrary)
      (else
        (GameplayTags|AddGameplayTag _charactertags "(TagName=\"CharacterStatus.Damageable\")" :!class /Script/GameplayTags.BlueprintGameplayTagLibrary)))))

(fn TakeDamage
  (params (Damage :type Float%20%28double-precision%29))
  (bind _playerhealthbar (Variables|Default|GetPlayerHealthBar))
  (if (GameplayTags|HasTag (Variables|/Game/Game/Blueprints/Characters/Master/BP_CharacterBase.BP_CharacterBase_C|GetCharacterTags (Variables|Default|GetOwner)) "(TagName=\"CharacterStatus.Damageable\")")
    (bind _output_get (Variables|Default|SetHealth (- (Variables|Default|GetHealth) Damage)))
    (Default|CallOnDamageTaken)
    (if (<= _output_get 0.0)
      (Default|CallOnDeath (Variables|Default|GetOwner)))
    (Utilities|IsValid _playerhealthbar
      (:Is%20Valid
        (Default|ChangeSliderValue _playerhealthbar (Variables|Default|GetHealth))))))

(fn Heal
  (params (HealAmount :type Float%20%28double-precision%29))
  (Variables|Default|SetHealth (Math|Float|Clamp(Float) (+ HealAmount (Variables|Default|GetHealth)) 0.0 (Variables|Default|GetMaxHealth)))
  (Default|ChangeSliderValue (Variables|Default|GetPlayerHealthBar) (Variables|Default|GetHealth)))