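; BP_Door is a door that slides by a Translation offset when a BP_CharacterBase enters its Box trigger and back when one leaves.
; Overlap events, bound on BeginPlay, play MoveSound, set NewPosition by adding or subtracting Translation, and restart the TranslationTime timeline.
; The timeline lerps the Mesh from its current location, not a stored origin, so overlaps during movement offset the resting position.
; A second Timeline graph is never run.
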(event `self.ReceiveBeginPlay`
  (bind _box (`self.Box`))
  (add `PrimitiveComponent.OnComponentBeginOverlap` _box (`|CreateDelegate` :!event `TriggerCollision`))
  (add `PrimitiveComponent.OnComponentEndOverlap` _box (`|CreateDelegate` :!event `EndCollision`)))

(event `TriggerCollision`
  (params (OverlappedComponent :type "PrimitiveComponent Object Reference") (OtherActor :type "Actor Object Reference") (OtherComp :type "PrimitiveComponent Object Reference") (OtherBodyIndex :type Integer) (bFromSweep :type Boolean) (SweepResult :type "HitResult Structure (by ref)"))
  (bind _mesh (`self.Mesh`))
  (bind _returnvalue (`SceneComponent.K2_GetComponentLocation` (`self.Mesh`)))
  (cast `/Game/Game/Blueprints/Characters/Master/BP_CharacterBase` OtherActor)
  (`GameplayStatics.PlaySoundAtLocation` (`self.MoveSound`) _returnvalue (struct) 1.0 1.0 0.0 null null null null)
  (set `self.NewPosition` (+ _returnvalue (`self.Translation`)))
  (bind (_direction _lerp) (`Timeline|TranslationTime` :!via `PlayFromStart` :!label _label)
    (:`Update`
      (`SceneComponent.K2_SetWorldLocation` _mesh (`KismetMathLibrary.VLerp` (`SceneComponent.K2_GetComponentLocation` _mesh) (`self.NewPosition`) _lerp) false false))))

(event `EndCollision`
  (params (OverlappedComponent :type "PrimitiveComponent Object Reference") (OtherActor :type "Actor Object Reference") (OtherComp :type "PrimitiveComponent Object Reference") (OtherBodyIndex :type Integer))
  (bind _returnvalue (`SceneComponent.K2_GetComponentLocation` (`self.Mesh`)))
  (cast `/Game/Game/Blueprints/Characters/Master/BP_CharacterBase` OtherActor)
  (`GameplayStatics.PlaySoundAtLocation` (`self.MoveSound`) _returnvalue (struct) 1.0 1.0 0.0 null null null null)
  (set `self.NewPosition` (- _returnvalue (`self.Translation`)))
  (goto _label :!via `PlayFromStart`))

(fn `UserConstructionScript`)