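; Trigger sphere actor that marks where the player can perform an execute and shows an execute prompt while in range.
; It creates a hidden W_Execute widget on BeginPlay and toggles its visibility as BP_Player enters or leaves the overlap.
; While overlapped, it binds to the player's OnExecuting event and relays it through its own OnExecutingSphere dispatcher.
; The construction script sizes ExecuteSphere from ExecuteRadius.
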(event `self.ReceiveBeginPlay`
  (bind _returnvalue (`|CreateWidget` "/Game/GameAssets/GameObjects/Widgets/HUD/W_Execute.W_Execute_C"))
  (bind _output_get (set `self.ExecuteWidget` _returnvalue))
  (`Widget.SetVisibility` _output_get "Hidden")
  (`UserWidget.AddToViewport` _output_get 0))

(event `self.ReceiveActorBeginOverlap`
  (params (OtherActor :type "Actor Object Reference"))
  (bind _asbp_player (cast `/Game/Game/Blueprints/Characters/Master/BP_Player` OtherActor))
  (set `self.OverlappedPlayer` _asbp_player)
  (`KismetSystemLibrary.PrintString` "PLAYER COLLIDING")
  (`Widget.SetVisibility` (`self.ExecuteWidget`) "Visible")
  (add `/Game/Game/Blueprints/Characters/Master/BP_Player.OnExecuting` (`self.OverlappedPlayer`) (delegate `CallExecuting`)))

(event `CallExecuting`
  (`self.OnExecutingSphere`))

(event `self.ReceiveActorEndOverlap`
  (params (OtherActor :type "Actor Object Reference"))
  (cast `/Game/Game/Blueprints/Characters/Master/BP_Player` OtherActor)
  (remove `/Game/Game/Blueprints/Characters/Master/BP_Player.OnExecuting` (`self.OverlappedPlayer`) (`|CreateDelegate` :!event `CallExecuting`))
  (set `self.OverlappedPlayer` null)
  (`Widget.SetVisibility` (`self.ExecuteWidget`) "Hidden"))

(fn `UserConstructionScript`
  (`SphereComponent.SetSphereRadius` (`self.ExecuteSphere`) (`self.ExecuteRadius`) true))