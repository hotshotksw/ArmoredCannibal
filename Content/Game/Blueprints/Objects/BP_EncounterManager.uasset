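; BP_EncounterManager is an actor that coordinates a group of enemies as one combat encounter.
; On BeginPlay it binds to each enemy's AI target-spotted and health damage and death delegates, with handlers to alert every AI controller or process a death.
; Deaths remove the enemy from the list, firing OnEncounterFinished when it empties.
; Otherwise, a delayed radio sound precedes a death-reaction voiceline chosen via random picks from remaining enemies.
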(event `self.ReceiveBeginPlay`
  (for _array_element (`self.Enemies`)
    (bind _output_get (set `self.CurrentEnemy` _array_element))
    (bind _asbp_aicontroller (cast `/Game/Game/Blueprints/Characters/Enemy/BP_AIController` (`AIBlueprintHelperLibrary.GetAIController` _output_get)))
    (add `/Game/Game/Blueprints/Characters/Enemy/BP_AIController.OnTargetSpotted` _asbp_aicontroller (`|CreateDelegate` :!event `AlertEnemies`))
    (add `/Game/Game/Blueprints/ActorComponents/HealthComponent.OnDamageTaken` (`/Game/Game/Blueprints/Characters/Master/BP_CharacterBase.HealthComponent` (`self.CurrentEnemy`)) (`|CreateDelegate` :!event `AlertEnemies`))
    (add `/Game/Game/Blueprints/ActorComponents/HealthComponent.OnDeath` (`/Game/Game/Blueprints/Characters/Master/BP_CharacterBase.HealthComponent` (`self.CurrentEnemy`)) (`|CreateDelegate` :!event `DeadEnemy`))))

(event `AlertEnemies`
  (for _array_element (`self.Enemies`)
    (bind _asbp_aicontroller (cast `/Game/Game/Blueprints/Characters/Enemy/BP_AIController` (`AIBlueprintHelperLibrary.GetAIController` _array_element)))
    (`/Game/Game/Blueprints/Characters/Enemy/BP_AIController.Alert` _asbp_aicontroller)))

(event `DeadEnemy`
  (params (DeadCharacter :type "/Game/Game/Blueprints/Characters/Master/BP_CharacterBase Object Reference"))
  (bind _enemies (`self.Enemies`))
  (bind _outitem (`KismetArrayLibrary.Array_Random` _enemies))
  (for _array_element (`self.Enemies`)
    (if (== DeadCharacter _array_element)
      (`KismetArrayLibrary.Array_RemoveItem` (`self.Enemies`) _array_element)
      (break)))
  (if (== (`KismetArrayLibrary.Array_Length` _enemies) 0)
    (`self.OnEncounterFinished`)
    (else
      (`/Engine/EditorBlueprintResources/StandardMacros.IsValid` _outitem
        (:`Is Valid`
          (`KismetSystemLibrary.Delay` 0.5)
          (`GameplayStatics.PlaySound2D` "/Game/Game/Audio/radio_on.radio_on" 0.5 1.0 0.0 null null)
          (`KismetSystemLibrary.Delay` 0.5)
          (`/Engine/EditorBlueprintResources/StandardMacros.IsValid` (`KismetArrayLibrary.Array_Random` (`/Game/Game/Blueprints/Characters/Master/BP_CharacterBase.OnCharacterDeath_Voicelines` _outitem))
            (:`Is Valid`
              (`GameplayStatics.PlaySound2D` null 1.0 1.0 0.0 null null)
              (`KismetSystemLibrary.PrintString` "AUDIO PLAYED"))))))))

(fn `UserConstructionScript`)