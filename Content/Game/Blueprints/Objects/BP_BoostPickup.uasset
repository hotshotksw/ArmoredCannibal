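; BP_BoostPickup is a pickup that gives an overlapping BP_Player a full MaxBoost worth of boost.
; On actor overlap it passes MaxBoost to ChangeBoostValue on the player's first BoostComponent, then toggles the Sphere's active state and hides it with its children.
; If DoesRegenerate is set, the Sphere is shown and toggled back after a fixed delay; otherwise the actor stays hidden without being destroyed.
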(event `self.ReceiveActorBeginOverlap`
  (params (OtherActor :type "Actor Object Reference"))
  (bind _sphere (`self.Sphere`))
  (bind _asbp_player (cast `/Game/Game/Blueprints/Characters/Master/BP_Player` OtherActor))
  (bind _returnvalue (`self.K2_GetComponentsByClass` _asbp_player "/Game/Game/Blueprints/ActorComponents/BoostComponent.BoostComponent_C"))
  (if (> (`KismetArrayLibrary.Array_Length` _returnvalue) 0)
    (bind _output (`|GetArrayItem` _returnvalue))
    (`/Game/Game/Blueprints/ActorComponents/BoostComponent.ChangeBoostValue` _output (`/Game/Game/Blueprints/ActorComponents/BoostComponent.MaxBoost` _output))
    (`ActorComponent.ToggleActive` _sphere)
    (`SceneComponent.SetVisibility` _sphere false true)
    (if (`self.DoesRegenerate`)
      (`KismetSystemLibrary.Delay` 10.0)
      (`SceneComponent.SetVisibility` _sphere true true)
      (`ActorComponent.ToggleActive` _sphere))))

(fn `UserConstructionScript`)